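; BP_Enemy_BasicAI is a basic AI enemy Blueprint that starts its behavior tree when play begins.
; On BeginPlay it checks for a valid AI controller, then runs the tree held in BTAsset on that controller.
; Tick and the construction script only call their parent versions, and the overlap event is disabled, so the Blueprint adds no other logic of its own.
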(event EventBeginPlay
  (bind _self self)
  (bind _returnvalue (AI|GetAIController _self))
  (Utilities|IsValid _returnvalue
    (:Is%20Valid
      (AI|RunBehaviorTree _returnvalue (Variables|Default|GetBTAsset)))))

(event Collision|EventActorBeginOverlap
  (params (OtherActor :type Actor%20Object%20Reference))
  (|CallParentFunction OtherActor) ; This node is disabled and will not be called.\nDrag off pins to build functionality.
)

(event EventTick
  (params (DeltaSeconds :type Float%20%28single-precision%29))
  (|CallParentFunction DeltaSeconds))

(fn ConstructionScript
  (|CallParentFunction))