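; Sandbox game mode for a wave-defense game, handling music, local split-screen setup and match start/end.
; BeginPlay reads the "players" option, builds single or split-screen UI (spawning a recolored second Babooshka for multiplayer), and blocks movement input.
; GameStart adds on-screen controls, restores movement and starts the map from its level data asset.
; Win/lose handlers show the GameState's end widget with sound; the intro animation and countdown call are disconnected.
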(event Custom|OnGameWin_Event_0
  (bind _returnvalue (Game|GetPlayerController 0))
  ;[1 1 1] OnGameWin UI
  (bind _aswave_defense_game_state_base (Utilities|Casting|CastToWaveDefenseGameStateBase (Game|GetGameState)))
  (Default|SetupwithGameState (Variables|/Game/GameModes/WaveDefense/WaveDefenseGameStateBase.WaveDefenseGameStateBase_C|GetGameEndWidget _aswave_defense_game_state_base) _aswave_defense_game_state_base)
  (Rendering|Components|TextRender|SetText (Variables|/Game/Widget/WBP_EndGame.WBP_EndGame_C|GetEndText (Variables|/Game/GameModes/WaveDefense/WaveDefenseGameStateBase.WaveDefenseGameStateBase_C|GetGameEndWidget _aswave_defense_game_state_base)) "You Win!")
  (UserInterface|Viewport|AddtoViewport (Variables|/Game/GameModes/WaveDefense/WaveDefenseGameStateBase.WaveDefenseGameStateBase_C|GetGameEndWidget _aswave_defense_game_state_base) 999)
  ;;[1 1 1] TODO: Make menu controllable by 1P controller
  (Input|DisableInput (Pawn|GetControlledPawn _returnvalue) _returnvalue)
  (Variables|/Script/Engine.PlayerController|SetbShowMouseCursor _returnvalue true)
  (Audio|PlaySound2D "/Game/Audio/SFX/Voice/Karen/karen_newhighscore_Cue.karen_newhighscore_Cue" 1.0 1.0 0.0 0 0))

(event Custom|OnGameLose_Event_0
  (bind _returnvalue (Game|GetPlayerController 0))
  ;[1 1 1] OnGameLose UI
  (bind _aswave_defense_game_state_base (Utilities|Casting|CastToWaveDefenseGameStateBase (Game|GetGameState)))
  (Default|SetupwithGameState (Variables|/Game/GameModes/WaveDefense/WaveDefenseGameStateBase.WaveDefenseGameStateBase_C|GetGameEndWidget _aswave_defense_game_state_base) _aswave_defense_game_state_base)
  (Rendering|Components|TextRender|SetText (Variables|/Game/Widget/WBP_EndGame.WBP_EndGame_C|GetEndText (Variables|/Game/GameModes/WaveDefense/WaveDefenseGameStateBase.WaveDefenseGameStateBase_C|GetGameEndWidget _aswave_defense_game_state_base)) "You Lose!")
  ;;[1 1 1] TODO: Make menu controllable by 1P controller
  (UserInterface|Viewport|AddtoViewport (Variables|/Game/GameModes/WaveDefense/WaveDefenseGameStateBase.WaveDefenseGameStateBase_C|GetGameEndWidget _aswave_defense_game_state_base) 999)
  (Variables|/Script/Engine.PlayerController|SetbShowMouseCursor _returnvalue true)
  (Input|DisableInput (Pawn|GetControlledPawn _returnvalue) _returnvalue)
  (Audio|PlaySound2D "/Game/Audio/SFX/Voice/Karen/karen-gameover_Cue.karen-gameover_Cue" 1.0 1.0 0.0 0 0))

(event Custom|GameStart
  (bind _returnvalue (UserInterface|CreateWidget "/Game/Widget/Widget_OnScreenControls.Widget_OnScreenControls_C"))
  (UserInterface|Viewport|AddtoViewport _returnvalue 0)
  (CallFunction|SetAllPlayerControllerInputActive true)
  (Class|UDSGameModeBase|StartGame (Variables|Default|GetMapLevelDataAsset))
  (Default|CallGameModeStart))

(event EventBeginPlay
  ;[1 1 1] BGM
  (bind _returnvalue (Audio|CreateSound2D "/Game/Audio/Music/gameplay_music.gameplay_music" 1.0 1.0 0.0 0))
  (bind _output_get (Variables|Default|SetGameplayBGM _returnvalue))
  (Audio|Components|Audio|Play _output_get 0.0)
  (bind _output_get_2 (Variables|Default|SetNumPlayers (Math|Conversions|ToInteger(Byte) (Class|GameplayStatics|ParseOption (Variables|Default|GetOptionsString) "players"))))
  (if (> _output_get_2 1)
    ;[1 1 1] Split Screen
    (Variables|Default|SetHUDClass "/Game/HUD/HUD_Gameplay_SplitScreen.HUD_Gameplay_SplitScreen_C")
    (bind _returnvalue_2 (Class|GameplayStatics|CreatePlayer -1))
    (bind _asbp_babooshka (Utilities|Casting|CastToBP_Babooshka (Pawn|GetControlledPawn _returnvalue_2)))
    (Rendering|Material|SetMaterialbyName (Variables|/Script/Engine.Character|GetMesh _asbp_babooshka) "babs_hood" "/Game/Materials/Characters/Babooshka_Hood2.Babooshka_Hood2")
    (bind _returnvalue_3 (UserInterface|CreateWidget (Variables|Default|GetSplitScreenGameplayWidget)))
    (UserInterface|Viewport|AddtoViewport _returnvalue_3 0)
    (else
      (bind _returnvalue_4 (UserInterface|CreateWidget (Variables|Default|GetSinglePlayerGameplayWidget)))
      (UserInterface|Viewport|AddtoViewport _returnvalue_4 0)))
  (CallFunction|SetAllPlayerControllerInputActive false)
  (EventDispatchers|AssignOnGameWin (delegate Custom|OnGameWin_Event_0))
  (EventDispatchers|AssignOnGameLose (delegate Custom|OnGameLose_Event_0)))

(fn ConstructionScript)

(fn StartGameMode
  (bind _aswave_defense_game_state_base (Utilities|Casting|CastToWaveDefenseGameStateBase (Game|GetGameState)))
  (EventDispatchers|BindEventtoWBPGameStartAnimationDone (Variables|/Game/GameModes/WaveDefense/WaveDefenseGameStateBase.WaveDefenseGameStateBase_C|GetGameStartWidget _aswave_defense_game_state_base) (EventDispatchers|CreateEvent :!event Custom|GameStart))
  (Default|Play (Variables|/Game/GameModes/WaveDefense/WaveDefenseGameStateBase.WaveDefenseGameStateBase_C|GetGameStartWidget _aswave_defense_game_state_base)))

(fn SetAllPlayerControllerInputActive
  (params (Enable :type Boolean))
  (bind _returnvalue (Class|GameModeBase|GetNumPlayers))
  (for _index (range 0 (- _returnvalue 1))
    (Input|SetIgnoreMoveInput (Game|GetPlayerController _index) (not Enable))))