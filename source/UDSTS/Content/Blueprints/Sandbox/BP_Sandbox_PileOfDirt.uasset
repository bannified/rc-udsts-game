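; Sandbox dirt pile actor that tints its sphere with CloudColor and repeatedly spawns random enemy units beneath itself.
; A looping SpawnRate timer asks the wave game state to spawn a random SpawnUnitAssets entry, then zeroes that enemy's Damage.
; ResetSpawnCoroutine restarts the timer.
; The counter increment and Matter-zeroing nodes are unconnected, so the MaxSpawnCount check never sees the count rise.
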(event EventBeginPlay
  (bind _cloudcolor (Variables|Default|GetCloudColor))
  (|CallParentFunction)
  (Rendering|Material|SetVectorParameterValueonMaterials (Variables|Default|GetSphere) "BaseColour" (Math|Vector|MakeVector (.r _cloudcolor) (.g _cloudcolor) (.b _cloudcolor)))
  (Variables|Default|SetCurrentSpawnCount 0)
  (Utilities|Time|SetTimerbyFunctionName self "SpawnRandomSpawnUnit" (Variables|Default|GetSpawnRate) true))

(event Collision|EventActorBeginOverlap
  (params (OtherActor :type Actor%20Object%20Reference))
  (|CallParentFunction OtherActor) ; This node is disabled and will not be called.\nDrag off pins to build functionality.
)

(event EventTick
  (params (DeltaSeconds :type Float%20%28single-precision%29))
  (|CallParentFunction DeltaSeconds) ; This node is disabled and will not be called.\nDrag off pins to build functionality.
)

(fn ConstructionScript
  (|CallParentFunction))

(fn SpawnRandomSpawnUnit
  (bind _spawnunitassets (Variables|Default|GetSpawnUnitAssets))
  (bind _asudsgame_mode_base (Utilities|Casting|CastToUDSGameModeBase (Game|GetGameMode)))
  (bind _aswave_game_mode_state (Utilities|Casting|CastToWaveGameModeState (Variables|/Script/UDSTS.UDSGameModeBase|GetCurrentState _asudsgame_mode_base)))
  (if (or (<= (Variables|Default|GetCurrentSpawnCount) (Variables|Default|GetMaxSpawnCount)) (< (Variables|Default|GetMaxSpawnCount) 0))
    (bind _returnvalue (Class|WaveGameModeState|SpawnwithSpawnUnitAssetatLocation _aswave_game_mode_state (Utilities|Array|Get(acopy) _spawnunitassets (Math|Random|RandomIntegerinRange 0 (- (Utilities|Array|Length _spawnunitassets) 1))) (+ (Transformation|GetActorLocation) "0, 0,-425.000000")))
    (bind _asenemy_base (Utilities|Casting|CastToEnemyBase _returnvalue))
    (Variables|/Script/UDSTS.EnemyBase|SetDamage _asenemy_base 0.0)))

(fn ResetSpawnCoroutine
  (Utilities|Time|ClearTimerbyFunctionName self "SpawnRandomSpawnUnit")
  (Utilities|Time|SetTimerbyFunctionName self "SpawnRandomSpawnUnit" (Variables|Default|GetSpawnRate) true))