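; Health component that tracks the current health and death state of whatever uses it.
; InitHealth sets the starting value and clears the dead flag.
; TakeDamage subtracts damage, or clamps health to zero, sets IsDead and calls the death event when the hit is lethal.
; It does not check IsDead first, so further hits at zero can fire death again; debug prints report each change.
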(event Custom|TakeDamage
  (params (Damage :type Float%20%28single-precision%29))
  (if (>= 0.0 (- (Variables|Default|GetCurrentHealth) Damage))
    ;[1 1 1] HP reaches 0
    (Variables|Default|SetCurrentHealth 0.0)
    (Variables|Default|SetisDead true)
    (Default|CallDeathEvent)
    (Development|PrintString "isDead")
    (else
      ;[1 1 1] Some HP remaining
      (bind _output_get (Variables|Default|SetCurrentHealth (- (Variables|Default|GetCurrentHealth) Damage)))
      (Development|PrintString (Utilities|String|ToString(Float) _output_get)))))

(event Custom|InitHealth
  (params (InitialHealth :type Float%20%28single-precision%29))
  (Variables|Default|SetCurrentHealth InitialHealth)
  (Variables|Default|SetisDead false)
  (Development|PrintString "Health initialized"))

(event EventBeginPlay)

(event EventTick
  (params (DeltaSeconds :type Float%20%28single-precision%29)))