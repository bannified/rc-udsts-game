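; Shop inventory Blueprint that sells base health upgrades and nozzle levels to a Customer, paid in matter from their Bag.
; DisplayWidget opens BP_ShopWidget with a self reference and UI-only input; Escape calls HideWidget to restore game input.
; Transact checks and deducts matter, gating UpgradeBase's addition to current health.
; BuyNozzle is provisional: it raises the level before calling Transact, ignores the result and always uses the first cost.
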(event Input|KeyboardEvents|Escape
  (params (Key :type Key%20Structure))
  (:Pressed
    (CallFunction|HideWidget)))

(fn ConstructionScript)

(fn DisplayWidget
  (bind _returnvalue (Game|GetPlayerController 0))
  (bind _returnvalue_2 (UserInterface|CreateWidget "/Game/Blueprints/Shop/BP_ShopWidget.BP_ShopWidget_C" (Game|GetPlayerController 0)))
  ;[1 1 1] Set ShopInventory for UI to access
  (Variables|/Game/Blueprints/Shop/BP_ShopWidget.BP_ShopWidget_C|SetShopInventory _returnvalue_2 self)
  (Variables|/Game/Blueprints/Shop/BP_ShopWidget.BP_ShopWidget_C|SetNozzleListSize _returnvalue_2 (Utilities|Array|Length (Variables|Default|GetNozzleInventoryList)))
  (bind _output_get (Variables|Default|SetShopInventoryWidget _returnvalue_2))
  (UserInterface|Viewport|AddtoViewport _output_get 0)
  (Input|SetInputModeUIOnly _returnvalue _returnvalue_2 "LockAlways")
  (Variables|/Script/Engine.PlayerController|SetbShowMouseCursor _returnvalue true))

(fn HideWidget
  (bind _returnvalue (Game|GetPlayerController 0))
  (Widget|RemovefromParent (Variables|Default|GetShopInventoryWidget))
  (Class|WidgetBlueprintLibrary|SetFocustoGameViewport)
  (Input|SetInputModeGameOnly _returnvalue)
  (Variables|/Script/Engine.PlayerController|SetbShowMouseCursor _returnvalue false))

(fn Transact
  (params (Cost :type Float%20%28single-precision%29))
  (bind _customer (Variables|Default|GetCustomer))
  (bind _bag (Variables|/Game/Blueprints/BP_Babooshka.BP_Babooshka_C|GetBag _customer))
  ;[1 1 1] Let characterbase handle transaction, if purchased -> true
  (bind _result (Default|IsMatterSufficient _bag Cost))
  (if _result
    (Default|ChangeMatterValueby _bag (* -1 Cost))
    (return _result)))

(fn UpgradeBase
  (params (UpgradeAmount :type Float%20%28single-precision%29) (Cost :type Float%20%28single-precision%29))
  (bind _base (Variables|Default|GetBase))
  (bind _bpc_health (Variables|/Game/Blueprints/BP_Base_Proto.BP_Base_Proto_C|GetBPC_Health _base))
  ;[1 1 1] Increase base health by upgrade amount [to update with new base in future]
  (bind _ispurchased (CallFunction|Transact Cost))
  (if _ispurchased
    (Variables|/Game/Blueprints/BPC_Health.BPC_Health_C|SetCurrentHealth _bpc_health (+ UpgradeAmount (Variables|/Game/Blueprints/BPC_Health.BPC_Health_C|GetCurrentHealth _bpc_health)))
    (Development|PrintString "Base upgraded")))

(fn BuyNozzle
  (params (Nozzle :type PDA%20Nozzle%20Object%20Reference))
  ;[1 1 1] TODO: Update after adding inventory bp
  (Math|Integer|IncrementInt (Variables|/Game/Blueprints/Weapon/PDA_Nozzle.PDA_Nozzle_C|GetCurrentLevel Nozzle)
    (:%20%20
      (CallFunction|Transact (Utilities|Array|Get(acopy) (Variables|/Game/Blueprints/Weapon/PDA_Nozzle.PDA_Nozzle_C|GetCost Nozzle))))))

(fn IsMatterSufficient
  (params (Required :type Float%20%28single-precision%29))
  (bind _result (Default|IsMatterSufficient (Variables|/Game/Blueprints/BP_Babooshka.BP_Babooshka_C|GetBag (Variables|Default|GetCustomer)) Required))
  (return _result))