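; BP_Shop_Placement is a placeable shop that BP_Babooshka characters can open when nearby.
; Overlapping EntryBox shows a per-player interact prompt, and pressing Interact inside it opens the inventory UI of the child-actor BP_ShopInventory.
; Leaving the separate ExitBox hides both the prompt and the inventory.
; The construction script caches that child inventory and passes it the shop's Base reference when valid.
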(event OnComponentBeginOverlap(EntryBox)
  (params (OverlappedComponent :type Primitive%20Component%20Object%20Reference) (OtherActor :type Actor%20Object%20Reference) (OtherComp :type Primitive%20Component%20Object%20Reference) (OtherBodyIndex :type Integer) (bFromSweep :type Boolean) (SweepResult :type Hit%20Result%20Structure%20%28by%20ref%29))
  ;[1 1 1] In proximity
  (bind _asbp_babooshka (Utilities|Casting|CastToBP_Babooshka OtherActor))
  (if (Class|PrimitiveComponent|IsOverlappingComponent (Variables|/Script/Engine.Character|GetCapsuleComponent _asbp_babooshka) (Variables|Default|GetEntryBox))
    (CallFunction|DisplayWidget _asbp_babooshka)))

(event OnComponentEndOverlap(ExitBox)
  (params (OverlappedComponent :type Primitive%20Component%20Object%20Reference) (OtherActor :type Actor%20Object%20Reference) (OtherComp :type Primitive%20Component%20Object%20Reference) (OtherBodyIndex :type Integer))
  ;[1 1 1] Not in proximity
  (bind _asbp_babooshka (Utilities|Casting|CastToBP_Babooshka OtherActor))
  (if (not (Class|PrimitiveComponent|IsOverlappingComponent (Variables|/Script/Engine.Character|GetCapsuleComponent _asbp_babooshka) (Variables|Default|GetExitBox)))
    (CallFunction|HideWidget _asbp_babooshka)
    (Default|HideWidget (Variables|Default|GetShopInventory) _asbp_babooshka)))

(event EventBeginPlay
  (bind _asbp_shop_inventory (Utilities|Casting|CastToBP_ShopInventory (Variables|/Script/Engine.ChildActorComponent|GetChildActor (Variables|Default|GetInventory))))
  (Variables|Default|SetShopInventory _asbp_shop_inventory))

(event Input|ActionEvents|InputActionInteract
  (params (Key :type Key%20Structure))
  ;[1 1 1] Character in proximity access shop
  (:Pressed
    (bind _asbp_babooshka (Utilities|Casting|CastToBP_Babooshka (stale OnComponentBeginOverlap(EntryBox) OtherActor)))
    (if (Class|PrimitiveComponent|IsOverlappingComponent (Variables|/Script/Engine.Character|GetCapsuleComponent _asbp_babooshka) (Variables|Default|GetEntryBox))
      (Default|DisplayWidget (Variables|Default|GetShopInventory) _asbp_babooshka)
      (Variables|Default|SetIsShopInvVisible true))))

(fn ConstructionScript
  (bind _asbp_shop_inventory (Utilities|Casting|CastToBP_ShopInventory (Variables|/Script/Engine.ChildActorComponent|GetChildActor (Variables|Default|GetInventory))))
  (Variables|Default|SetShopInventory _asbp_shop_inventory)
  (bind _base (Variables|Default|GetBase)
    (:then
      (Variables|/Game/Blueprints/Shop/BP_ShopInventory.BP_ShopInventory_C|SetBase _asbp_shop_inventory _base))
    (:else)))

(fn HideWidget
  (params (Owning%20Player :type BP%20Babooshka%20Object%20Reference))
  (bind _shopinteractwidget (Variables|/Game/Blueprints/BP_Babooshka.BP_Babooshka_C|GetShopInteractWidget Owning%20Player)
    (:then
      (Widget|RemovefromParent _shopinteractwidget))
    (:else)))

(fn DisplayWidget
  (params (OwningPlayer :type BP%20Babooshka%20Object%20Reference))
  (bind _asplayer_controller (Utilities|Casting|CastToPlayerController (Pawn|GetController OwningPlayer)))
  (bind _returnvalue (UserInterface|CreateWidget "/Game/Blueprints/Shop/BP_InteractWidget.BP_InteractWidget_C" _asplayer_controller))
  (Variables|/Game/Blueprints/BP_Babooshka.BP_Babooshka_C|SetShopInteractWidget OwningPlayer _returnvalue)
  (bind _output_get (Variables|Default|SetInteractWidget _returnvalue))
  (UserInterface|Viewport|AddtoViewport _output_get 0))