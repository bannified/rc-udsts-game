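; Shop inventory that sells nozzles and base health repairs to players, paid with matter from the customer's Bag.
; DisplayWidget creates a per-player BP_ShopWidget, disables movement and enables cursor input, while HideWidget removes it and restores Swimming movement and game-only input.
; BuyNozzle prices by the customer's owned level and UpgradeBase heals only a damaged Base, both charging through Transact before applying the effect.
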(event Input|KeyboardEvents|Escape
  (params (Key :type Key%20Structure))
  (:Pressed
    (CallFunction|HideWidget)))

(fn ConstructionScript)

(fn DisplayWidget
  (params (Owning%20Player :type BP%20Babooshka%20Object%20Reference))
  (bind _asplayer_controller (Utilities|Casting|CastToPlayerController (Pawn|GetController Owning%20Player)))
  (bind _returnvalue (UserInterface|CreateWidget "/Game/Blueprints/Shop/BP_ShopWidget.BP_ShopWidget_C" _asplayer_controller))
  (Variables|/Game/Blueprints/BP_Babooshka.BP_Babooshka_C|SetShopInventoryWidget Owning%20Player _returnvalue)
  (Variables|/Game/Blueprints/Shop/BP_ShopWidget.BP_ShopWidget_C|SetNozzleListSize _returnvalue (Utilities|Array|Length (Variables|Default|GetNozzleInventoryList)))
  (bind _output_get (Variables|Default|SetShopInventoryWidget _returnvalue))
  (Variables|/Game/Blueprints/Shop/BP_ShopWidget.BP_ShopWidget_C|SetShopInventory _returnvalue self)
  (Variables|/Game/Blueprints/Shop/BP_ShopWidget.BP_ShopWidget_C|SetTargetCustomer _returnvalue Owning%20Player)
  (UserInterface|Viewport|AddtoPlayerScreen _output_get 20)
  (Default|Init _output_get Owning%20Player)
  (Pawn|Components|CharacterMovement|DisableMovement (Variables|/Script/Engine.Character|GetCharacterMovement Owning%20Player))
  (Variables|/Game/Blueprints/BP_Babooshka.BP_Babooshka_C|SetIsInUI Owning%20Player true)
  (Input|SetInputModeGameandUI _asplayer_controller _returnvalue "DoNotLock" true)
  (Variables|/Game/Blueprints/Shop/BP_ShopWidget.BP_ShopWidget_C|SetTargetCustomer _returnvalue Owning%20Player)
  (Variables|/Script/Engine.PlayerController|SetbShowMouseCursor _asplayer_controller true))

(fn HideWidget
  (params (Owning%20Player :type BP%20Babooshka%20Object%20Reference))
  (bind _shopinventorywidget (Variables|/Game/Blueprints/BP_Babooshka.BP_Babooshka_C|GetShopInventoryWidget Owning%20Player)
    (:then
      (Widget|RemovefromParent _shopinventorywidget))
    (:else
      _))
  (bind _asplayer_controller (Utilities|Casting|CastToPlayerController (Pawn|GetController Owning%20Player)))
  (Pawn|Components|CharacterMovement|SetMovementMode (Variables|/Script/Engine.Character|GetCharacterMovement Owning%20Player) "MOVE_Swimming" 0)
  (Variables|/Game/Blueprints/BP_Babooshka.BP_Babooshka_C|SetIsInUI Owning%20Player false)
  (Class|WidgetBlueprintLibrary|SetFocustoGameViewport)
  (Input|SetInputModeGameOnly _asplayer_controller)
  (Variables|/Script/Engine.PlayerController|SetbShowMouseCursor _asplayer_controller false))

(fn Transact
  (params (Cost :type Float%20%28single-precision%29) (Customer :type BP%20Babooshka%20Object%20Reference))
  (bind _bag (Variables|/Game/Blueprints/BP_Babooshka.BP_Babooshka_C|GetBag Customer))
  ;[1 1 1] Let characterbase handle transaction, if purchased -> true
  (bind _result (Default|IsMatterSufficient _bag Cost))
  (if _result
    (Default|ChangeMatterValueby _bag (* -1 Cost))
    (return _result)
    (else
      (return false))))

(fn UpgradeBase
  (params (UpgradeAmount :type Float%20%28single-precision%29) (Cost :type Float%20%28single-precision%29) (Customer :type BP%20Babooshka%20Object%20Reference))
  (bind _base (Variables|Default|GetBase))
  (bind _healthcomponent (Variables|/Script/UDSTS.Base|GetHealthComponent _base))
  ;[1 1 1] Increase base health by upgrade amount [to update with new base in future]
  (if (not (>= (Variables|/Script/UDSTS.HealthComponent|GetcurrentHealth _healthcomponent) (Variables|/Script/UDSTS.HealthComponent|GetmaxHealth _healthcomponent)))
    (bind _ispurchased (CallFunction|Transact Cost Customer))
    (if _ispurchased
      (Class|HealthComponent|AlterHealth _healthcomponent UpgradeAmount))))

(fn BuyNozzle
  (params (Customer :type BP%20Babooshka%20Object%20Reference) (Nozzle :type PDA%20Nozzle%20Object%20Reference))
  (bind _nozzletolevellist (Variables|/Game/Blueprints/BP_Babooshka.BP_Babooshka_C|GetNozzleToLevelList Customer))
  (bind _cost (Variables|/Game/Blueprints/Weapon/PDA_Nozzle.PDA_Nozzle_C|GetCost Nozzle))
  (if (Utilities|Map|Contains _nozzletolevellist Nozzle)
    ;[1 1 1] Upgrade, already has nozzle
    (bind _ispurchased (CallFunction|Transact (Utilities|Array|Get(acopy) _cost (+ (.Value (Utilities|Map|Find _nozzletolevellist Nozzle)) 1)) Customer))
    (if _ispurchased
      (Default|TransferNozzle Customer Nozzle :!label _label)
      (else
        (Development|PrintString "Not enough matter" :!label _label_2)))
    (else
      ;[1 1 1] First time purchase
      (bind _ispurchased_2 (CallFunction|Transact (Utilities|Array|Get(acopy) _cost) Customer))
      (if _ispurchased_2
        (goto _label)
        (else
          (goto _label_2))))))

(fn IsMatterSufficient
  (params (Required :type Float%20%28single-precision%29) (Customer :type BP%20Babooshka%20Object%20Reference))
  (bind _result (Default|IsMatterSufficient (Variables|/Game/Blueprints/BP_Babooshka.BP_Babooshka_C|GetBag Customer) Required))
  (return _result))