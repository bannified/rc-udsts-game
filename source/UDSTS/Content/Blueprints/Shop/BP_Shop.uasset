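; BP_Shop is a shop actor that lets the BP_Babooshka character open a shop inventory when nearby.
; Overlap events add an interact prompt widget on entry, then remove it and hide ShopInventory on exit.
; Pressing Interact while the character overlaps the Box displays ShopInventory and then sets that character as its Customer.
; On BeginPlay, the shop passes its Base reference to ShopInventory.
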(event EventBeginPlay
  (Variables|/Game/Blueprints/Shop/BP_ShopInventory.BP_ShopInventory_C|SetBase (Variables|Default|GetShopInventory) (Variables|Default|GetBase)))

(event Collision|EventActorBeginOverlap
  (params (OtherActor :type Actor%20Object%20Reference))
  ;[1 1 1] In proximity
  (if (== (Utilities|GetClass OtherActor) "/Game/Blueprints/BP_Babooshka.BP_Babooshka_C")
    (CallFunction|DisplayWidget)))

(event Collision|EventActorEndOverlap
  (params (OtherActor :type Actor%20Object%20Reference))
  ;[1 1 1] Not in proximity
  (if (== (Utilities|GetClass OtherActor) "/Game/Blueprints/BP_Babooshka.BP_Babooshka_C")
    (CallFunction|HideWidget)
    (Default|HideWidget (Variables|Default|GetShopInventory))))

(event Input|ActionEvents|InputActionInteract
  (params (Key :type Key%20Structure))
  (bind _shopinventory (Variables|Default|GetShopInventory))
  ;[1 1 1] Character in proximity access shop
  (:Pressed
    (if (Collision|IsOverlappingActor (Variables|Default|GetBox) (stale Collision|EventActorBeginOverlap OtherActor) :!class /Script/Engine.PrimitiveComponent)
      (Default|DisplayWidget _shopinventory)
      (bind _asbp_babooshka (Utilities|Casting|CastToBP_Babooshka (stale Collision|EventActorBeginOverlap OtherActor)))
      (bind _output_get (Variables|Default|SetCustomer _asbp_babooshka))
      (Variables|/Game/Blueprints/Shop/BP_ShopInventory.BP_ShopInventory_C|SetCustomer _shopinventory _output_get))))

(fn ConstructionScript)

(fn HideWidget
  (Widget|RemovefromParent (Variables|Default|GetInteractWidget)))

(fn DisplayWidget
  (bind _returnvalue (UserInterface|CreateWidget "/Game/Blueprints/Shop/BP_InteractWidget.BP_InteractWidget_C"))
  (bind _output_get (Variables|Default|SetInteractWidget _returnvalue))
  (UserInterface|Viewport|AddtoViewport _output_get 0))