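; BP_PlasticBottle_dup is a plastic bottle enemy Blueprint that follows a waypoint network under AI control.
; When its capsule overlaps a BP_Waypoint, it asks that waypoint for a random next waypoint.
; It writes that waypoint and its location to the WaypointObject and TargetDestination Blackboard keys.
; BeginPlay, Tick and construction only call the parent class.
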(event OnComponentBeginOverlap(CapsuleComponent)
  (params (OverlappedComponent :type Primitive%20Component%20Object%20Reference) (OtherActor :type Actor%20Object%20Reference) (OtherComp :type Primitive%20Component%20Object%20Reference) (OtherBodyIndex :type Integer) (bFromSweep :type Boolean) (SweepResult :type Hit%20Result%20Structure%20%28by%20ref%29))
  (bind _self self)
  (bind _returnvalue (AI|GetBlackboard _self))
  ;[1 1 1] Waypoint Collision
  (bind _asbp_waypoint (Utilities|Casting|CastToBP_Waypoint OtherActor))
  (bind _newparam (Default|GetRandomWaypoint _asbp_waypoint))
  (AI|Components|Blackboard|SetValueasObject _returnvalue (Utilities|Name|MakeLiteralName "WaypointObject") _newparam)
  (AI|Components|Blackboard|SetValueasVector _returnvalue (Utilities|Name|MakeLiteralName "TargetDestination") (Transformation|GetActorLocation _newparam)))

(event EventTick
  (params (DeltaSeconds :type Float%20%28single-precision%29))
  (|CallParentFunction DeltaSeconds))

(event EventBeginPlay
  (|CallParentFunction))

(fn ConstructionScript
  (|CallParentFunction))