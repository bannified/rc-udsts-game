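; Plastic bottle enemy pawn that runs a behavior tree and turns to align with its movement.
; On BeginPlay it runs the assigned behavior tree on its AI controller, spawning a default controller first if none exists.
; Each Tick, when Y velocity is nonzero, it sets yaw from the arctangent of Y/X velocity plus a half turn.
; The single-argument arctangent does not distinguish opposite headings.
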(event EventBeginPlay
  (bind _self self)
  (bind _returnvalue (AI|GetAIController _self))
  (Utilities|IsValid _returnvalue
    (:Is%20Valid
      (AI|RunBehaviorTree _returnvalue (Variables|Default|GetUnitBehaviorTreeAsset)))
    (:Is%20Not%20Valid
      (Pawn|SpawnDefaultController)
      (bind _asaicontroller (Utilities|Casting|CastToAIController (Pawn|GetController)))
      (AI|RunBehaviorTree _asaicontroller (Variables|Default|GetUnitBehaviorTreeAsset)))))

(event Collision|EventActorBeginOverlap
  (params (OtherActor :type Actor%20Object%20Reference)))

(event EventTick
  (params (DeltaSeconds :type Float%20%28single-precision%29))
  (bind _floatingpawnmovement (Variables|Default|GetFloatingPawnMovement))
  (bind _velocity (Variables|/Script/Engine.MovementComponent|GetVelocity _floatingpawnmovement))
  (if (!= (.y _velocity) 0.0)
    (Transformation|SetActorRotation (Math|Vector|RotatorfromAxisandAngle "0, 0,1.000000" (+ (Class|KismetMathLibrary|DegAtan (/ (.y _velocity) (.x _velocity))) 1.8e+02)) true)))

(fn ConstructionScript)