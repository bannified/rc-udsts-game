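; Toxic Blob enemy that attacks the shark base with projectiles and flees from Babooshka, driven through AI blackboard keys.
; Tick checks range and line of sight to the base, setting CanSeeBase, and faces it once ShootAtBase has fired.
; Seeing or being damaged by Babooshka switches to fleeing speed, hopping between random linked waypoints on overlap.
; Once the player is far enough away, it restores speed and resets the base-targeting keys.
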(event OnComponentBeginOverlap(CapsuleComponent)
  (params (OverlappedComponent :type Primitive%20Component%20Object%20Reference) (OtherActor :type Actor%20Object%20Reference) (OtherComp :type Primitive%20Component%20Object%20Reference) (OtherBodyIndex :type Integer) (bFromSweep :type Boolean) (SweepResult :type Hit%20Result%20Structure%20%28by%20ref%29))
  (bind _self self)
  (bind _returnvalue (AI|GetBlackboard _self))
  ;[1 1 1] Waypoint Collision
  (if (ScalableFloat|GetValueasBool (AI|GetBlackboard self) (Utilities|Name|MakeLiteralName "IsFleeing"))
    (bind _asbp_waypoint (Utilities|Casting|CastToBP_Waypoint OtherActor))
    (bind _newparam (Default|GetRandomWaypoint _asbp_waypoint))
    (AI|Components|Blackboard|SetValueasObject _returnvalue (Utilities|Name|MakeLiteralName "WaypointObject") _newparam)
    (AI|Components|Blackboard|SetValueasVector _returnvalue (Utilities|Name|MakeLiteralName "TargetDestination") (Transformation|GetActorLocation _newparam))))

(event OnSeePawn(PawnSensing)
  (params (Pawn :type Pawn%20Object%20Reference))
  (bind _asbp_babooshka (Utilities|Casting|CastToBP_Babooshka Pawn))
  (CallFunction|ToggleFlee _asbp_babooshka))

(event EventTick
  (params (DeltaSeconds :type Float%20%28single-precision%29))
  (|CallParentFunction DeltaSeconds)
  (if (Variables|Default|GetIsShooting)
    (Transformation|SetActorRotation (Math|Rotator|FindLookatRotation (Transformation|GetActorLocation) (Variables|Default|GetBaseLocation))))
  (if (ScalableFloat|GetValueasBool (AI|GetBlackboard (AI|GetAIController self)) (Utilities|Name|MakeLiteralName "IsFleeing"))
    (CallFunction|CheckPlayerDistance)
    (else
      (CallFunction|CheckBaseLOS))))

(event Game|Damage|EventAnyDamage
  (params (Damage :type Float%20%28single-precision%29) (DamageType :type Damage%20Type%20Object%20Reference) (InstigatedBy :type Controller%20Object%20Reference) (DamageCauser :type Actor%20Object%20Reference))
  (if (not (Variables|Default|GetIsFleeing))
    (bind _asbp_babooshka (Utilities|Casting|CastToBP_Babooshka DamageCauser))
    (CallFunction|ToggleFlee _asbp_babooshka)))

(event EventBeginPlay
  (|CallParentFunction)
  (AI|Components|Blackboard|SetValueasBool (AI|GetBlackboard (AI|GetAIController self)) (Utilities|Name|MakeLiteralName "IsFleeing") false)
  (Variables|Default|SetBaseMaxSpeed (Variables|Default|GetMovementSpeed)))

(fn ConstructionScript
  (|CallParentFunction))

(fn CheckBaseLOS
  (bind _self self)
  (bind _self_2 self)
  (bind _asactor (Utilities|Casting|CastToActor (AI|Components|Blackboard|GetValueasObject (AI|GetBlackboard _self) (Utilities|Name|MakeLiteralName "BaseObject"))))
  (if (Controller|LineOfSightTo (AI|GetAIController _self) _asactor (Transformation|GetWorldLocation (Variables|Default|GetShootingPoint)) false)
    (Utilities|Casting|CastToBP_SharkBase _asactor)
    (if (<= (Transformation|GetDistanceTo _self_2 _asactor) (Variables|Default|GetRangeToShoot))
      (AI|Components|Blackboard|SetValueasBool (AI|GetBlackboard _self_2) (Utilities|Name|MakeLiteralName "CanSeeBase") true)
      (Variables|Default|SetBaseLocation (Transformation|GetActorLocation _asactor))
      (return true)
      (else
        (return false)))))

(fn CheckArc
  (bind _self self)
  (Class|GameplayStatics|BlueprintPredictProjectilePathbyTraceChannel (Transformation|GetActorLocation _self) (+ (Transformation|GetActorForwardVector _self) (Transformation|GetActorUpVector _self)) true 1.0 "ECC_WorldStatic" false (Utilities|Array|MakeArray _self) "ForOneFrame" 0.5 15.0 2.0 1.0))

(fn ShootatBase
  (bind _returnvalue (Game|SpawnActorfromClass "/Game/Blueprints/Enemies/ToxicBlob/BP_ToxicProjectile.BP_ToxicProjectile_C" (Transformation|GetWorldTransform (Variables|Default|GetShootingPoint)) "AlwaysSpawn" 0 0))
  (Default|InitDirection _returnvalue (Transformation|GetWorldLocation (Variables|Default|GetCapsuleComponent)) (AI|Components|Blackboard|GetValueasVector (AI|GetBlackboard (AI|GetAIController self)) (Utilities|Name|MakeLiteralName "TargetDestination")))
  (Variables|Default|SetIsShooting true))

(fn ToggleFlee
  (params (PlayerObject :type Pawn%20Object%20Reference))
  (bind _self self)
  (bind _returnvalue (AI|GetAIController _self))
  (bind _returnvalue_2 (AI|GetBlackboard _returnvalue))
  (Variables|Default|SetIsFleeing true)
  (AI|Components|Blackboard|SetValueasBool _returnvalue_2 (Utilities|Name|MakeLiteralName "IsFleeing") true)
  (AI|Components|Blackboard|SetValueasObject _returnvalue_2 (Utilities|Name|MakeLiteralName "PlayerObject") PlayerObject)
  (Variables|Default|SetPlayerPawn PlayerObject)
  (Variables|Default|SetIsShooting false)
  (Variables|/Script/Engine.FloatingPawnMovement|SetMaxSpeed (Variables|Default|GetFloatingPawnMovement) (Variables|Default|GetFleeingSpeed))
  (Variables|Default|SetMovementSpeed (Variables|Default|GetFleeingSpeed)))

(fn CheckPlayerDistance
  (bind _self self)
  (bind _basemaxspeed (Variables|Default|GetBaseMaxSpeed))
  (bind _returnvalue (AI|GetAIController _self))
  (bind _returnvalue_2 (AI|GetBlackboard _returnvalue))
  (if (>= (Transformation|GetDistanceTo self (Variables|Default|GetPlayerPawn)) 2e+03)
    (AI|Components|Blackboard|SetValueasBool _returnvalue_2 (Utilities|Name|MakeLiteralName "IsFleeing") false)
    (AI|Components|Blackboard|SetValueasBool _returnvalue_2 (Utilities|Name|MakeLiteralName "CanSeeBase") false)
    (AI|Components|Blackboard|SetValueasBool _returnvalue_2 (Utilities|Name|MakeLiteralName "HasSetBase") false)
    (Variables|Default|SetMovementSpeed _basemaxspeed)
    (Variables|/Script/Engine.FloatingPawnMovement|SetMaxSpeed (Variables|Default|GetFloatingPawnMovement) _basemaxspeed)
    (Variables|Default|SetIsFleeing false)))