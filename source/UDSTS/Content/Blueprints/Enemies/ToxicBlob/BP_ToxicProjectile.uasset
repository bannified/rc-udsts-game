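; BP_ToxicProjectile is a ToxicBlob enemy projectile that flies in a straight line and destroys itself on hitting the player base.
; InitDirection stores a unit vector between two given points, and Tick sweeps the actor a fixed step along it each frame, independent of delta time.
; A sphere hit destroys the projectile only if the other actor is a BP_Base_Proto; damage is still an unimplemented placeholder.
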(event OnComponentHit(Sphere)
  (params (HitComponent :type Primitive%20Component%20Object%20Reference) (OtherActor :type Actor%20Object%20Reference) (OtherComp :type Primitive%20Component%20Object%20Reference) (NormalImpulse :type Vector :default "0, 0, 0") (Hit :type Hit%20Result%20Structure%20%28by%20ref%29))
  ;[1 1 1] On collide with base, Deal damage  (IMPLEMENT THIS!)
  (Utilities|Casting|CastToBP_Base_Proto OtherActor)
  (Actor|DestroyActor))

(event EventBeginPlay)

(event Collision|EventActorBeginOverlap
  (params (OtherActor :type Actor%20Object%20Reference)))

(event EventTick
  (params (DeltaSeconds :type Float%20%28single-precision%29))
  (Transformation|SetActorLocation (+ (Transformation|GetWorldLocation (Variables|Default|GetDefaultSceneRoot)) (* (Variables|Default|GetMoveDirection) 7.0)) true false))

(fn ConstructionScript)

(fn InitDirection
  (params (From :type Vector) (To :type Vector))
  (Variables|Default|SetMoveDirection (Math|Vector|GetUnitDirection(Vector) From To)))