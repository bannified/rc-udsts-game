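; SUA_EnemyBase initializes an EnemyBase unit with its configured stats and optional AI override.
; InitializeUnit, noted as running after the actor's BeginPlay, casts the actor and copies movement speed, maximum and starting health, and Matter onto it and its components.
; When a behavior tree override is valid, it replaces the unit's tree asset and runs it on the enemy's AI controller.
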(event EventInitializeUnit
  (params (Actor :type Actor%20Object%20Reference))
  (bind _behaviourtreeoverride (Variables|Default|GetBehaviourTreeOverride))
  ;[1 1 1] NOTE: InitiliazeUnit is called AFTER the Actor's BeginPlay()
  (bind _asenemy_base (Utilities|Casting|CastToEnemyBase Actor))
  ;;[1 1 1] Movement
  (Variables|/Script/Engine.FloatingPawnMovement|SetMaxSpeed (Variables|/Script/UDSTS.UnitBase|GetFloatingPawnMovement _asenemy_base) (Variables|Default|GetMovementSpeed))
  ;;[1 1 1] HealthComponent
  (Variables|/Script/UDSTS.HealthComponent|SetmaxHealth (Variables|/Script/UDSTS.UnitBase|GetHealthComponent _asenemy_base) (Variables|Default|GetMaxHealth))
  (Variables|/Script/UDSTS.HealthComponent|SetstartingHealth (Variables|/Script/UDSTS.UnitBase|GetHealthComponent _asenemy_base) (Variables|Default|GetStartingHealth))
  ;;[1 1 1] Matter
  (Variables|/Script/UDSTS.EnemyBase|SetMatter _asenemy_base (Variables|Default|GetMatter))
  ;;[1 1 1] BehaviourTree overriding (only runs if it exists)
  (Utilities|IsValid _behaviourtreeoverride
    (:Is%20Valid
      (bind _output_get (Variables|/Script/UDSTS.UnitBase|SetUnitBehaviorTreeAsset _asenemy_base _behaviourtreeoverride))
      (AI|RunBehaviorTree (AI|GetAIController _asenemy_base) _output_get))))