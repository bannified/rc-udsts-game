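; Base floating enemy that runs a behavior tree and registers on each BP_Babooshka player's position indicator.
; Randomly offset timelines drive roll, bobbing and speed variation, while Tick turns it toward its velocity and its healthbar toward player 0's camera.
; Damage triggers a hurt mask and sound, and health changes update the healthbar, hidden at full health.
; Death by a BP_Babooshka awards Matter and destroys the actor, spawning a death effect.
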(event OnDeathEvent(HealthComponent)
  (params (Victim :type Actor%20Object%20Reference) (Killer :type Actor%20Object%20Reference))
  ;[1 1 1] Reward Matter To Player
  (bind _asbp_babooshka (Utilities|Casting|CastToBP_Babooshka Killer))
  (Default|ChangeMatterValueby (Variables|/Game/Blueprints/BP_Babooshka.BP_Babooshka_C|GetBag _asbp_babooshka) (Variables|Default|GetMatter))
  (Audio|SpawnSoundatLocation (Variables|Default|GetDeathSound) "0, 0, 0" "0, 0, 0" 1.0 1.0 0.0 0 0)
  (Actor|DestroyActor))

(event Custom|ApplyHurtMaskEvent
  (bind _audiocomponent (Variables|Default|GetAudioComponent))
  ;[1 1 1] Hurt Mask Application
  (if (not (Variables|Default|GetIsMaskApplied))
    (Variables|Default|SetIsMaskApplied true)
    (Audio|Components|Audio|SetSound _audiocomponent (Variables|Default|GetHurtSound))
    (Audio|Components|Audio|Play _audiocomponent 0.0)
    (bind _newtrack_0 (Timeline|Timeline_1 PlayFromStart)
      (:Update
        (Rendering|Material|SetScalarParameterValueonMaterials (Variables|Default|GetMainMesh) "Alpha" _newtrack_0))
      (:Finished
        (Variables|Default|SetIsMaskApplied false)))))

(event Custom|OnHealthChanged_Event_0
  (params (HealthComp :type Health%20Component%20Object%20Reference) (health :type Float%20%28single-precision%29) (healthDelta :type Float%20%28single-precision%29) (DamageType :type Damage%20Type%20Object%20Reference) (InstigatedBy :type Controller%20Object%20Reference) (DamageCauser :type Actor%20Object%20Reference))
  ;[1 1 1] Bind Healthbar Update
  (CallFunction|SetHealthbarVisibilityBasedonHealth)
  (CallFunction|SetHealthBarPercentage))

(event Custom|TriggerDeathEffectEvent
  (params (DestroyedActor :type Actor%20Object%20Reference))
  ;[1 1 1] Bind DeathEffectEvent
  (Effects|SpawnEmitteratLocation "/Game/ParticleEffects/PES_EnemyDead.PES_EnemyDead" (Transformation|GetActorLocation DestroyedActor)))

(event Custom|OnTakeAnyDamage_Event_1
  (params (DamagedActor :type Actor%20Object%20Reference) (Damage :type Float%20%28single-precision%29) (DamageType :type Damage%20Type%20Object%20Reference) (InstigatedBy :type Controller%20Object%20Reference) (DamageCauser :type Actor%20Object%20Reference))
  ;[1 1 1] Bind HurtEvent
  (if (> Damage 0.0)
    (CallFunction|ApplyHurtMaskEvent)))

(event EventBeginPlay
  (bind _self self)
  (bind _returnvalue (AI|GetAIController _self))
  ;[1 1 1] Run BehaviourTree
  (Utilities|IsValid _returnvalue
    (:Is%20Valid
      (AI|RunBehaviorTree _returnvalue (Variables|Default|GetUnitBehaviorTreeAsset)))
    (:Is%20Not%20Valid
      (Pawn|SpawnDefaultController)
      (bind _asaicontroller (Utilities|Casting|CastToAIController (Pawn|GetController)))
      (AI|RunBehaviorTree _asaicontroller (Variables|Default|GetUnitBehaviorTreeAsset))))
  (bind _spawnsound (Variables|Default|GetSpawnSound)
    (:then
      (Audio|PlaySound2D _spawnsound 1.0 1.0 0.0 0 0))
    (:else
      _))
  ;[1 1 1] Bind HurtEvent
  (EventDispatchers|AssignOnTakeAnyDamage (delegate Custom|OnTakeAnyDamage_Event_1))
  ;[1 1 1] Bind Healthbar Update
  (EventDispatchers|AssignOnHealthChanged (Variables|Default|GetHealthComponent) (delegate Custom|OnHealthChanged_Event_0))
  ;[1 1 1] Bind DeathEffectEvent
  (EventDispatchers|BindEventtoOnDestroyed (delegate Custom|TriggerDeathEffectEvent))
  ;[1 1 1] Register to Enemy Position Screen of each Player
  (bind _returnvalue_2 (Class|GameModeBase|GetNumPlayers (Game|GetGameMode)))
  (for _index (range 0 (- _returnvalue_2 1))
    (bind _asbp_babooshka (Utilities|Casting|CastToBP_Babooshka (Game|Player|GetPlayerPawn _index)))
    (Default|AddActortoScreen (Variables|/Game/Blueprints/BP_Babooshka.BP_Babooshka_C|GetEnemiesPositionIndicator _asbp_babooshka) self (Variables|Default|GetPositionIndicatorSprite)))
  (Utilities|FlowControl|Sequence
    (:then_0
      ;[1 1 1] RotationAnim
      (bind _rotationvalue (Timeline|RotationAnim SetNewTime)
        (:Update
          (Transformation|AddActorLocalRotation (Math|Rotator|MakeRotator (* _rotationvalue (Variables|Default|GetRotationAnimMultiplier)) 0.0 0.0) false false)
          ;[1 1 1] VelocityAnim
          (bind _velocityvalue (Timeline|VelocityAnim Play)
            (:Update
              (Variables|/Script/Engine.FloatingPawnMovement|SetMaxSpeed (Variables|Default|GetFloatingPawnMovement) (+ (* _velocityvalue (Variables|Default|GetVelocityAnimRange)) (Variables|Default|GetMovementSpeed))))))))
    (:then_1
      ;[1 1 1] BobbingAnim
      (bind _upwardbobbingvalue (Timeline|BobbingAnim SetNewTime)
        (:Update
          (Transformation|AddActorLocalOffset (Math|Vector|MakeVector 0.0 0.0 (* _upwardbobbingvalue (Variables|Default|GetBobbingAnimMultiplier))) true false)
          (Timeline|RotationAnim Play))))
    (:then_2
      (Timeline|VelocityAnim SetNewTime))))

(event EventTick
  (params (DeltaSeconds :type Float%20%28single-precision%29))
  (bind _self self)
  (bind _capsulecomponent (Variables|Default|GetCapsuleComponent _self))
  (bind _returnvalue (Transformation|GetWorldLocation _capsulecomponent))
  (Transformation|SetActorRotation (Math|Interpolation|RInterpTo (Transformation|GetActorRotation self) (Math|Rotator|FindLookatRotation _returnvalue (+ _returnvalue (Math|Vector|Normalize (Variables|/Script/Engine.MovementComponent|GetVelocity (Variables|Default|GetFloatingPawnMovement))))) (Variables|Default|GetRInterpDeltaTime) (Variables|Default|GetRInterpSpeed)))
  (CallFunction|RotateHealthbartoFacePlayer)
  ;[1 1 1] BobbingAnim
  (bind _upwardbobbingvalue (Timeline|BobbingAnim Play)
    (:Update
      (Transformation|AddActorLocalOffset (Math|Vector|MakeVector 0.0 0.0 (* _upwardbobbingvalue (Variables|Default|GetBobbingAnimMultiplier))) true false)
      ;[1 1 1] RotationAnim
      (bind _rotationvalue (Timeline|RotationAnim Play)
        (:Update
          (Transformation|AddActorLocalRotation (Math|Rotator|MakeRotator (* _rotationvalue (Variables|Default|GetRotationAnimMultiplier)) 0.0 0.0) false false)
          ;[1 1 1] VelocityAnim
          (bind _velocityvalue (Timeline|VelocityAnim Play)
            (:Update
              (Variables|/Script/Engine.FloatingPawnMovement|SetMaxSpeed (Variables|Default|GetFloatingPawnMovement) (+ (* _velocityvalue (Variables|Default|GetVelocityAnimRange)) (Variables|Default|GetMovementSpeed))))))))))

(fn ConstructionScript)

(fn SetHealthBarPercentage
  (bind _healthcomponent (Variables|Default|GetHealthComponent))
  (bind _aswidget_healthbar (Utilities|Casting|CastToWidget_Healthbar (UserInterface|GetUserWidgetObject (Variables|Default|GetHealthbar))))
  (Default|SetHealthBarPercentageas _aswidget_healthbar (/ (Variables|/Script/UDSTS.HealthComponent|GetcurrentHealth _healthcomponent) (Variables|/Script/UDSTS.HealthComponent|GetmaxHealth _healthcomponent))))

(fn RotateHealthbartoFacePlayer
  (bind _returnvalue (Game|GetPlayerCameraManager 0))
  (bind _healthbaranchor (Variables|Default|GetHealthbarAnchor))
  (bind _returnvalue_2 (Transformation|GetActorLocation _returnvalue))
  (bind _returnvalue_3 (Transformation|GetWorldLocation _healthbaranchor))
  (bind _returnvalue_4 (Math|Rotator|FindLookatRotation _returnvalue_3 _returnvalue_2))
  (bind _healthbaranchor_2 (Variables|Default|GetHealthbarAnchor)
    (:then
      (Transformation|SetWorldRotation _healthbaranchor_2 (Math|Rotator|MakeRotator (.roll _returnvalue_4) (.pitch _returnvalue_4) (.yaw _returnvalue_4)) false false))
    (:else)))

(fn SetHealthbarVisibilityBasedonHealth
  (bind _healthcomponent (Variables|Default|GetHealthComponent))
  (Rendering|SetVisibility (Variables|Default|GetHealthbar) (not (>= (Variables|/Script/UDSTS.HealthComponent|GetcurrentHealth _healthcomponent) (Variables|/Script/UDSTS.HealthComponent|GetmaxHealth _healthcomponent))) false))