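; Oil tank enemy that patrols waypoints, charges a spotted character and knocks the Babooshka back on contact.
; Pawn sensing raises its speed and feeds the target to the Blackboard, with position updated each tick until it leaves range and base speed returns.
; While no target is seen, waypoint overlaps write the next waypoint to the Blackboard.
; Suck damage is countered by adding the amount back to health.
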(event OnSeePawn(PawnSensing)
  (params (Pawn :type Pawn%20Object%20Reference))
  (bind _self self)
  (bind _chargespeed (Variables|Default|GetChargeSpeed))
  (bind _returnvalue (AI|GetAIController _self))
  (bind _returnvalue_2 (AI|GetBlackboard _returnvalue))
  ;[1 1 1] OnSeePawn - Set PlayePawn Ref + BBKeys
  (bind _ascharacter_base (Utilities|Casting|CastToCharacterBase Pawn))
  (AI|Components|Blackboard|SetValueasBool _returnvalue_2 (Utilities|Name|MakeLiteralName "CanSeePlayer") true)
  (AI|Components|Blackboard|SetValueasObject _returnvalue_2 (Utilities|Name|MakeLiteralName "PlayerPawn") _ascharacter_base)
  (Variables|Default|SetCanSeePlayer true)
  (Variables|Default|SetPlayerPawn _ascharacter_base)
  (Variables|/Script/Engine.FloatingPawnMovement|SetMaxSpeed (Variables|Default|GetFloatingPawnMovement) _chargespeed)
  (Variables|Default|SetMovementSpeed _chargespeed))

(event OnComponentBeginOverlap(CapsuleComponent)
  (params (OverlappedComponent :type Primitive%20Component%20Object%20Reference) (OtherActor :type Actor%20Object%20Reference) (OtherComp :type Primitive%20Component%20Object%20Reference) (OtherBodyIndex :type Integer) (bFromSweep :type Boolean) (SweepResult :type Hit%20Result%20Structure%20%28by%20ref%29))
  (bind _self self)
  (bind _returnvalue (AI|GetBlackboard _self))
  ;[1 1 1] Waypoint Collision
  (if (not (Variables|Default|GetCanSeePlayer))
    (bind _asbp_waypoint (Utilities|Casting|CastToBP_Waypoint OtherActor))
    (AI|Components|Blackboard|SetValueasObject _returnvalue (Utilities|Name|MakeLiteralName "WaypointObject") (Variables|/Game/Blueprints/BP_Waypoint.BP_Waypoint_C|GetNextWaypoint _asbp_waypoint))
    (AI|Components|Blackboard|SetValueasVector _returnvalue (Utilities|Name|MakeLiteralName "TargetDestination") (Transformation|GetActorLocation (Variables|/Game/Blueprints/BP_Waypoint.BP_Waypoint_C|GetNextWaypoint _asbp_waypoint)))))

(event OnComponentHit(CapsuleComponent)
  (params (HitComponent :type Primitive%20Component%20Object%20Reference) (OtherActor :type Actor%20Object%20Reference) (OtherComp :type Primitive%20Component%20Object%20Reference) (NormalImpulse :type Vector :default "0, 0, 0") (Hit :type Hit%20Result%20Structure%20%28by%20ref%29))
  (bind _floatingpawnmovement (Variables|Default|GetFloatingPawnMovement))
  ;[1 1 1] Pushing the old lady
  (bind _ascharacter_base (Utilities|Casting|CastToCharacterBase OtherActor))
  (bind _asbp_babooshka (Utilities|Casting|CastToBP_Babooshka _ascharacter_base))
  (if (Variables|Default|GetCanSeePlayer)
    (Utilities|FlowControl|DoOnce false :!label _label
      (:Completed
        (Default|PushedBack _asbp_babooshka (Math|Vector|GetUnitDirection(Vector) (Transformation|GetActorLocation self) (Transformation|GetActorLocation _asbp_babooshka)) 1e+03)
        (Variables|/Script/Engine.MovementComponent|SetVelocity _floatingpawnmovement (* (Variables|/Script/Engine.MovementComponent|GetVelocity _floatingpawnmovement) 0.5))
        (Utilities|FlowControl|Delay 0.1)
        (goto _label Reset)))))

(event EventTick
  (params (DeltaSeconds :type Float%20%28single-precision%29))
  (|CallParentFunction DeltaSeconds)
  ;[1 1 1] Check player and position
  (if (Variables|Default|GetCanSeePlayer)
    (CallFunction|ChangeBBPlayerPosition)
    (CallFunction|CheckPlayerDistance)))

(event Game|Damage|EventAnyDamage
  (params (Damage :type Float%20%28single-precision%29) (DamageType :type Damage%20Type%20Object%20Reference) (InstigatedBy :type Controller%20Object%20Reference) (DamageCauser :type Actor%20Object%20Reference))
  (bind _healthcomponent (Variables|Default|GetHealthComponent))
  ;[1 1 1] Ignore sucks
  (Utilities|Casting|CastToDamageType_Suck DamageType)
  (Variables|/Script/UDSTS.HealthComponent|SetcurrentHealth _healthcomponent (+ (Variables|/Script/UDSTS.HealthComponent|GetcurrentHealth _healthcomponent) Damage)))

(event EventBeginPlay
  (|CallParentFunction)
  (Variables|Default|SetBaseMaxSpeed (Variables|Default|GetMovementSpeed)))

(fn ConstructionScript
  (|CallParentFunction))

(fn ChangeBBPlayerPosition
  (AI|Components|Blackboard|SetValueasVector (AI|GetBlackboard self) (Utilities|Name|MakeLiteralName "PlayerPawnPosition") (Transformation|GetActorLocation (Variables|Default|GetPlayerPawn))))

(fn CheckPlayerDistance
  (bind _self self)
  (bind _basemaxspeed (Variables|Default|GetBaseMaxSpeed))
  (if (not (< (Transformation|GetDistanceTo (Variables|Default|GetPlayerPawn) _self) 1024.0))
    (Variables|Default|SetCanSeePlayer false)
    (Variables|Default|SetPlayerPawn 0)
    (AI|Components|Blackboard|SetValueasBool (AI|GetBlackboard _self) (Utilities|Name|MakeLiteralName "CanSeePlayer") false)
    (Variables|/Script/Engine.FloatingPawnMovement|SetMaxSpeed (Variables|Default|GetFloatingPawnMovement) _basemaxspeed)
    (Variables|Default|SetMovementSpeed _basemaxspeed)))