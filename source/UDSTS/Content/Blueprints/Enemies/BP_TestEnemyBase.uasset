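; BP_TestEnemyBase is a test enemy that damages the base on contact.
; On BeginPlay it runs its assigned behavior tree through its AI controller, prints its name, and destroys itself after a fixed delay.
; When its main mesh begins overlapping a BP_Base, it deals damage through that base's HealthComponent and destroys itself.
; A look-at rotation toward the AI focus actor is present but unconnected.
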(event OnComponentBeginOverlap(MainMesh)
  (params (OverlappedComponent :type Primitive%20Component%20Object%20Reference) (OtherActor :type Actor%20Object%20Reference) (OtherComp :type Primitive%20Component%20Object%20Reference) (OtherBodyIndex :type Integer) (bFromSweep :type Boolean) (SweepResult :type Hit%20Result%20Structure%20%28by%20ref%29))
  (bind _asbp_base (Utilities|Casting|CastToBP_Base OtherActor))
  (Class|HealthComponent|TakeDamage (Variables|/Script/UDSTS.Base|GetHealthComponent _asbp_base) 1e+01)
  (Actor|DestroyActor))

(event EventBeginPlay
  (bind _asaicontroller (Utilities|Casting|CastToAIController (Pawn|GetController self))
    (:then
      (AI|RunBehaviorTree _asaicontroller (Variables|Default|GetUnitBehaviorTreeAsset))
      (Development|PrintString (Utilities|GetDisplayName self))
      (Utilities|FlowControl|Delay 1e+01)
      (Actor|DestroyActor))
    (:CastFailed
      (Development|PrintString "Aicontroller failed"))))

(event Collision|EventActorBeginOverlap
  (params (OtherActor :type Actor%20Object%20Reference)))

(event EventTick
  (params (DeltaSeconds :type Float%20%28single-precision%29)))

(fn ConstructionScript)