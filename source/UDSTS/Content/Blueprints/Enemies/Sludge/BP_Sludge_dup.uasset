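; Sludge enemy that roams between random waypoints and charges the player on sight or after surviving suck damage.
; It drives its AI through blackboard keys, updating player position each tick and dropping aggro at range after a short post-aggro grace delay.
; Hitting BP_Babooshka slows her and destroys the sludge.
; Blow damage splits it into small sludges, spawned through the wave game mode state and launched away from the damage causer.
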(event OnSeePawn(PawnSensing)
  (params (Pawn :type Pawn%20Object%20Reference))
  ;[1 1 1] OnSeePawn - Set PlayePawn Ref + BBKeys
  (if (not (Variables|Default|GetCanSeePlayer))
    (CallFunction|AggroPlayer Pawn)))

(event OnComponentBeginOverlap(CapsuleComponent)
  (params (OverlappedComponent :type Primitive%20Component%20Object%20Reference) (OtherActor :type Actor%20Object%20Reference) (OtherComp :type Primitive%20Component%20Object%20Reference) (OtherBodyIndex :type Integer) (bFromSweep :type Boolean) (SweepResult :type Hit%20Result%20Structure%20%28by%20ref%29))
  (bind _self self)
  (bind _returnvalue (AI|GetBlackboard _self))
  ;[1 1 1] Waypoint Collision
  (if (not (Variables|Default|GetCanSeePlayer))
    (bind _asbp_waypoint (Utilities|Casting|CastToBP_Waypoint OtherActor))
    (bind _newparam (Default|GetRandomWaypoint _asbp_waypoint))
    (AI|Components|Blackboard|SetValueasObject _returnvalue (Utilities|Name|MakeLiteralName "WaypointObject") _newparam)
    (AI|Components|Blackboard|SetValueasVector _returnvalue (Utilities|Name|MakeLiteralName "TargetDestination") (Transformation|GetActorLocation _newparam))))

(event OnComponentHit(CapsuleComponent)
  (params (HitComponent :type Primitive%20Component%20Object%20Reference) (OtherActor :type Actor%20Object%20Reference) (OtherComp :type Primitive%20Component%20Object%20Reference) (NormalImpulse :type Vector :default "0, 0, 0") (Hit :type Hit%20Result%20Structure%20%28by%20ref%29))
  ;[1 1 1] Slowing grandma
  (bind _ascharacter_base (Utilities|Casting|CastToCharacterBase OtherActor))
  (bind _asbp_babooshka (Utilities|Casting|CastToBP_Babooshka _ascharacter_base))
  (Default|SlowedDown _asbp_babooshka (Variables|Default|GetSlowSpeed) (Variables|Default|GetSlowDuration))
  (Actor|DestroyActor))

(event EventTick
  (params (DeltaSeconds :type Float%20%28single-precision%29))
  (|CallParentFunction DeltaSeconds)
  ;[1 1 1] Change BBKey to PlayerPos
  (if (Variables|Default|GetCanSeePlayer)
    (CallFunction|ChangeBBPlayerPosition)
    (if (Variables|Default|GetWasAggroed)
      (Utilities|FlowControl|Delay 1.0)
      (Variables|Default|SetWasAggroed false)
      (else
        (CallFunction|CheckPlayerDistance)))))

(event Game|Damage|EventAnyDamage
  (params (Damage :type Float%20%28single-precision%29) (DamageType :type Damage%20Type%20Object%20Reference) (InstigatedBy :type Controller%20Object%20Reference) (DamageCauser :type Actor%20Object%20Reference))
  (Utilities|Casting|CastToDamageType_Blow DamageType
    (:then
      (CallFunction|SplittoChildren (* (Math|Vector|GetUnitDirection(Vector) (Transformation|GetActorLocation DamageCauser) (Transformation|GetActorLocation self)) (Variables|Default|GetSplitForce))))
    (:CastFailed
      (Utilities|Casting|CastToDamageType_Suck DamageType)
      (bind _asbp_babooshka (Utilities|Casting|CastToBP_Babooshka DamageCauser))
      (if (not (<= (Variables|/Script/UDSTS.HealthComponent|GetcurrentHealth (Variables|Default|GetHealthComponent)) Damage))
        (CallFunction|AggroPlayer _asbp_babooshka)))))

(event EventBeginPlay
  (|CallParentFunction)
  (Variables|Default|SetBaseMaxSpeed (Variables|Default|GetMovementSpeed)))

(fn ConstructionScript
  (|CallParentFunction))

(fn ChangeBBPlayerPosition
  (AI|Components|Blackboard|SetValueasVector (AI|GetBlackboard self) (Utilities|Name|MakeLiteralName "PlayerPawnPosition") (Transformation|GetActorLocation (Variables|Default|GetPlayerPawn))))

(fn CheckPlayerDistance
  (bind _self self)
  (bind _basemaxspeed (Variables|Default|GetBaseMaxSpeed))
  (if (not (< (Transformation|GetDistanceTo (Variables|Default|GetPlayerPawn) _self) 1024.0))
    (Variables|Default|SetCanSeePlayer false)
    (Variables|Default|SetPlayerPawn 0)
    (AI|Components|Blackboard|SetValueasBool (AI|GetBlackboard _self) (Utilities|Name|MakeLiteralName "CanSeePlayer") false)
    (Variables|/Script/Engine.FloatingPawnMovement|SetMaxSpeed (Variables|Default|GetFloatingPawnMovement) _basemaxspeed)
    (Variables|Default|SetMovementSpeed _basemaxspeed)))

(fn SplittoChildren
  (params (Impulse :type Vector))
  (for _index (range 0 (- (Variables|Default|GetSplitCount) 1))
    (bind _asudsgame_mode_base (Utilities|Casting|CastToUDSGameModeBase (Game|GetGameMode)))
    (bind _aswave_game_mode_state (Utilities|Casting|CastToWaveGameModeState (Variables|/Script/UDSTS.UDSGameModeBase|GetCurrentState _asudsgame_mode_base)))
    (bind _returnvalue (Class|WaveGameModeState|SpawnwithSpawnUnitAssetatLocation _aswave_game_mode_state (Variables|Default|GetSplitSpawnUnit) (Transformation|GetActorLocation self)))
    (bind _asbp_sludge_small (Utilities|Casting|CastToBP_Sludge_Small _returnvalue))
    (Default|AddImpulseonSpawn _asbp_sludge_small Impulse))
  (Actor|DestroyActor))

(fn AggroPlayer
  (params (Pawn :type Pawn%20Object%20Reference))
  (bind _self self)
  (bind _chargespeed (Variables|Default|GetChargeSpeed))
  (bind _returnvalue (AI|GetAIController _self))
  (bind _returnvalue_2 (AI|GetBlackboard _returnvalue))
  (bind _ascharacter_base (Utilities|Casting|CastToCharacterBase Pawn))
  (AI|Components|Blackboard|SetValueasBool _returnvalue_2 (Utilities|Name|MakeLiteralName "CanSeePlayer") true)
  (AI|Components|Blackboard|SetValueasObject _returnvalue_2 (Utilities|Name|MakeLiteralName "PlayerPawn") _ascharacter_base)
  (Variables|Default|SetCanSeePlayer true)
  (Variables|Default|SetPlayerPawn _ascharacter_base)
  (Variables|/Script/Engine.FloatingPawnMovement|SetMaxSpeed (Variables|Default|GetFloatingPawnMovement) _chargespeed)
  (Variables|Default|SetMovementSpeed _chargespeed)
  (Variables|Default|SetWasAggroed true))