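; Player controller Blueprint that provides Ctrl+Alt number-key cheat shortcuts for debugging the game.
; Movement and weapon cheats loop over every player's pawn, restoring input and swimming movement or resetting BP_Babooshka nozzles to the basic level-zero weapon.
; World cheats destroy all EnemyBase actors and restore every Base's health.
; Flow cheats force unpause, open the main menu, or trigger the win through UDSGameModeBase.
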(event Input|KeyboardEvents|CtrlAlt8
  (params (Key :type Key%20Structure))
  ;[1 1 1] Reset all weapons, equip basic weapon lvl 0
  (:Pressed
    (bind _returnvalue (Class|GameModeBase|GetNumPlayers (Game|GetGameMode)))
    (for _index (range 0 (- _returnvalue 1))
      (bind _asbp_babooshka (Utilities|Casting|CastToBP_Babooshka (Pawn|GetControlledPawn (Game|GetPlayerController _index))))
      (Variables|/Game/Blueprints/BP_Babooshka.BP_Babooshka_C|SetNozzleToLevelList _asbp_babooshka (Utilities|Map|MakeMap))
      (Variables|/Game/Blueprints/BP_Babooshka.BP_Babooshka_C|SetNozzleList _asbp_babooshka (Utilities|Array|MakeArray))
      (Default|SetNozzleProperties (Variables|/Game/Blueprints/BP_Babooshka.BP_Babooshka_C|GetWeapon _asbp_babooshka) "/Game/GameplayData/Nozzles/PDA_Basic.PDA_Basic")
      (Utilities|Array|AddUnique (Variables|/Game/Blueprints/BP_Babooshka.BP_Babooshka_C|GetNozzleList _asbp_babooshka) "/Game/GameplayData/Nozzles/PDA_Basic.PDA_Basic")
      (Utilities|Map|Add (Variables|/Game/Blueprints/BP_Babooshka.BP_Babooshka_C|GetNozzleToLevelList _asbp_babooshka) "/Game/GameplayData/Nozzles/PDA_Basic.PDA_Basic" 0))))

(event Input|KeyboardEvents|CtrlAlt0
  (params (Key :type Key%20Structure))
  ;[1 1 1] Calls Win Game (Goes to win screen)
  (:Pressed
    (bind _asudsgame_mode_base (Utilities|Casting|CastToUDSGameModeBase (Game|GetGameMode)))
    (Class|UDSGameModeBase|WinGame _asudsgame_mode_base)))

(event Input|KeyboardEvents|CtrlAlt4
  (params (Key :type Key%20Structure))
  ;[1 1 1] Enable all Player's movement
  (:Pressed
    (bind _returnvalue (Class|GameModeBase|GetNumPlayers (Game|GetGameMode)))
    (for _index (range 0 (- _returnvalue 1))
      (Input|EnableInput (Pawn|GetControlledPawn (Game|GetPlayerController _index)) (Game|GetPlayerController _index))
      (bind _ascharacter_movement_component (Utilities|Casting|CastToCharacterMovementComponent (Pawn|GetMovementComponent (Pawn|GetControlledPawn (Game|GetPlayerController _index)))))
      (Pawn|Components|CharacterMovement|SetMovementMode _ascharacter_movement_component "MOVE_Swimming" 0)
      (Variables|/Script/Engine.CharacterMovementComponent|SetMaxSwimSpeed _ascharacter_movement_component 6e+02)
      (Input|SetInputModeGameandUI (Game|GetPlayerController _index) 0 "DoNotLock" false))
    (Development|PrintString "CHEAT: All Players' movement enabled")))

(event Input|KeyboardEvents|CtrlAlt5
  (params (Key :type Key%20Structure))
  ;[1 1 1] Destroy All Enemies
  (:Pressed
    (bind _outactors (Actor|GetAllActorsOfClass "/Script/UDSTS.EnemyBase"))
    (bind _arrayelement (Utilities|Array|ReverseforEachLoop _outactors)
      (:LoopBody
        (Utilities|IsValid _arrayelement
          (:Is%20Valid
            (Actor|DestroyActor _arrayelement))))
      (:Completed
        (Development|PrintString "CHEAT: All Enemies Destroyed")))))

(event Input|KeyboardEvents|CtrlAlt6
  (params (Key :type Key%20Structure))
  ;[1 1 1] Skip to Main Menu
  (:Pressed
    (Game|OpenLevel(byName) "MainMenu")))

(event Input|KeyboardEvents|CtrlAlt7
  (params (Key :type Key%20Structure))
  ;[1 1 1] Force Unpause
  (:Pressed
    (Game|SetGamePaused false)))

(event Input|KeyboardEvents|CtrlAlt9
  (params (Key :type Key%20Structure))
  ;[1 1 1] Resetting health of all bases
  (:Pressed
    (bind _outactors (Actor|GetAllActorsOfClass "/Script/UDSTS.Base"))
    (for _array_element _outactors
      (Class|HealthComponent|InitHealth (Variables|/Script/UDSTS.Base|GetHealthComponent _array_element) (Variables|/Script/UDSTS.HealthComponent|GetmaxHealth (Variables|/Script/UDSTS.Base|GetHealthComponent _array_element))))))

(fn ConstructionScript)