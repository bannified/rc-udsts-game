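; Oil tank AI unit, named as a healthbar test, that runs a behavior tree and carries a world healthbar.
; While Y velocity is non-zero, Tick yaws it along its movement and updates the bar's visibility, camera-relative rotation and fill.
; The fill divides current health by itself, so it never reflects damage.
; On death, a BP_Babooshka killer's bag receives its Matter and the tank is destroyed; other killers trigger neither.
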(event OnDeathEvent(HealthComponent)
  (params (Victim :type Actor%20Object%20Reference) (Killer :type Actor%20Object%20Reference))
  (bind _asbp_babooshka (Utilities|Casting|CastToBP_Babooshka Killer))
  (Default|ChangeMatterValueby (Variables|/Game/Blueprints/BP_Babooshka.BP_Babooshka_C|GetBag _asbp_babooshka) (Variables|Default|GetMatter))
  (Actor|DestroyActor))

(event EventBeginPlay
  (bind _self self)
  (bind _returnvalue (AI|GetAIController _self))
  (Utilities|IsValid _returnvalue
    (:Is%20Valid
      (AI|RunBehaviorTree _returnvalue (Variables|Default|GetUnitBehaviorTreeAsset)))
    (:Is%20Not%20Valid
      (Pawn|SpawnDefaultController)
      (bind _asaicontroller (Utilities|Casting|CastToAIController (Pawn|GetController)))
      (AI|RunBehaviorTree _asaicontroller (Variables|Default|GetUnitBehaviorTreeAsset)))))

(event Collision|EventActorBeginOverlap
  (params (OtherActor :type Actor%20Object%20Reference)))

(event EventTick
  (params (DeltaSeconds :type Float%20%28single-precision%29))
  (bind _floatingpawnmovement (Variables|Default|GetFloatingPawnMovement))
  (bind _velocity (Variables|/Script/Engine.MovementComponent|GetVelocity _floatingpawnmovement))
  (if (!= (.y _velocity) 0.0)
    (Transformation|SetActorRotation (Math|Vector|RotatorfromAxisandAngle "0, 0,1.000000" (+ (Class|KismetMathLibrary|DegAtan (/ (.y _velocity) (.x _velocity))) 1.8e+02)) true)
    ;[1 1 1] Healthbar Management
    (CallFunction|SetHealthbarVisibilityBasedonHealth)
    (CallFunction|RotateHealthbartoFacePlayer)
    (CallFunction|SetHealthbarPercentage)))

(fn ConstructionScript)

(fn SetHealthbarVisibilityBasedonHealth
  (bind _healthcomponent (Variables|Default|GetHealthComponent))
  (Rendering|SetVisibility (Variables|Default|GetHealthbar) (not (Math|Float|NearlyEqual(Float) (Variables|/Script/UDSTS.HealthComponent|GetmaxHealth _healthcomponent) (Variables|/Script/UDSTS.HealthComponent|GetcurrentHealth _healthcomponent) 0.001)) false))

(fn RotateHealthbartoFacePlayer
  (bind _returnvalue (Game|GetPlayerCameraManager 0))
  (bind _healthbaranchor (Variables|Default|GetHealthbarAnchor))
  (bind _returnvalue_2 (Transformation|GetActorLocation _returnvalue))
  (bind _returnvalue_3 (Transformation|GetWorldLocation _healthbaranchor))
  (bind _returnvalue_4 (Math|Rotator|FindLookatRotation _returnvalue_2 _returnvalue_3))
  (Transformation|SetWorldRotation (Variables|Default|GetHealthbarAnchor) (Math|Rotator|MakeRotator (.roll _returnvalue_4) (.pitch _returnvalue_4) (+ (.yaw _returnvalue_4) 1.8e+02)) false false))

(fn SetHealthbarPercentage
  (bind _healthcomponent (Variables|Default|GetHealthComponent))
  (bind _aswidget_healthbar (Utilities|Casting|CastToWidget_Healthbar (UserInterface|GetUserWidgetObject (Variables|Default|GetHealthbar))))
  (Default|SetHealthBarPercentageas _aswidget_healthbar (/ (Variables|/Script/UDSTS.HealthComponent|GetcurrentHealth _healthcomponent) (Variables|/Script/UDSTS.HealthComponent|GetcurrentHealth _healthcomponent))))