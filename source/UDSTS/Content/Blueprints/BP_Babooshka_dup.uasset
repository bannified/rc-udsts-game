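; Babooshka player character, a grandma armed with a vacuum weapon and back-mounted bag that gains matter from kills.
; Spawns and attaches weapon, nozzle and bag, creating per-player crosshair, nozzle-switch and enemy-indicator widgets on possession.
; Tick traces from the camera to aim weapon colliders and flag enemies in range, while looping timers drive firing.
; Also handles cycling and leveling nozzles, input routing to shop UI, jamming, swim slowdown and pushback.
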(event Custom|OnBoostActivated_Event_0
  (params (Charater :type Character%20Base%20Object%20Reference))
  ;[1 1 1] Boost Particle Effect
  (Effects|SpawnEmitterAttached (Variables|Default|GetBoosterParticleSystem) (Variables|/Game/Blueprints/Weapon/BP_VacuumBag.BP_VacuumBag_C|GetVacuumBag (Variables|Default|GetBag)) (Variables|Default|GetBoosterEndSocketName) "0, 0, 0" "0, 0, 0" (Variables|Default|GetBoosterParticleScale) "KeepRelativeOffset" true "AutoRelease")
  (Default|PlayBoostSound (Variables|Default|GetBag)))

(event Custom|SlowedDown
  (params (TempSpeed :type Float%20%28single-precision%29) (Delay :type Float%20%28single-precision%29))
  (bind _charactermovement (Variables|Character|GetCharacterMovement))
  ;[1 1 1] Slowing Grandma
  (if (Variables|Default|GetIsSlowed)
    (if (> (Variables|/Script/Engine.CharacterMovementComponent|GetMaxSwimSpeed _charactermovement) TempSpeed)
      (Variables|/Script/Engine.CharacterMovementComponent|SetMaxSwimSpeed _charactermovement TempSpeed :!label _label))
    (else
      (goto _label)))
  (Utilities|FlowControl|RetriggerableDelay 0.2)
  (Variables|/Script/Engine.CharacterMovementComponent|SetMaxSwimSpeed (Variables|Character|GetCharacterMovement) 6e+02))

(event Custom|JamWeapon
  (params (Duration :type Float%20%28single-precision%29))
  ;[1 1 1] Jam Weapon
  (Variables|Default|SetIsWeaponJammed true)
  (Variables|Default|SetbUseControllerRotationYaw false)
  ;;[1 1 1] Stop Shooting
  (Utilities|Time|ClearTimerbyFunctionName (Variables|Default|GetWeapon) "Primary")
  (Components|Activation|Deactivate (Variables|Default|GetPES_BubbleSucking))
  (Variables|Default|SetIsFiring false)
  (Animation|StopAnimMontage "/Game/Meshes/Characters/Babooshka_Resized/AMontage_Sucking_Babooshka.AMontage_Sucking_Babooshka")
  (Audio|Components|Audio|Stop (Variables|Default|GetWeaponAudio))
  (Utilities|FlowControl|Delay Duration)
  (Variables|Default|SetIsWeaponJammed false))

(event EventBeginPlay
  (CallFunction|InitWeapon)
  (CallFunction|InitVacuumBag)
  (EventDispatchers|AssignOnBoostActivated (delegate Custom|OnBoostActivated_Event_0)))

(event EventTick
  (params (DeltaSeconds :type Float%20%28single-precision%29))
  (bind _maincamera (Variables|Default|GetMainCamera))
  (bind _returnvalue (Transformation|GetWorldLocation _maincamera))
  ;[1 1 1] Linetrace to Crosshair
  (bind _outhit (Collision|LineTraceForObjects _returnvalue (+ _returnvalue (* (Math|Vector|GetForwardVector _maincamera) 5000)) (Variables|Default|GetEnemyType) false 0 "None"))
  ;[1 1 1] Update Weapon Collider Rotation
  (Transformation|SetWorldRotation (Variables|Default|GetWeaponColliders) (Math|Rotator|MakeRotator (.roll (Math|Rotator|FindLookatRotation (Transformation|GetWorldLocation (Variables|Character|GetMesh)) (.TraceEnd (|GetActorAndTraceEnd _outhit)))) (.pitch (Math|Rotator|FindLookatRotation (Transformation|GetWorldLocation (Variables|Character|GetMesh)) (.TraceEnd (|GetActorAndTraceEnd _outhit)))) (.yaw (Math|Rotator|FindLookatRotation (Transformation|GetWorldLocation (Variables|Character|GetMesh)) (.TraceEnd (|GetActorAndTraceEnd _outhit))))) false false)
  ;[1 1 1] Update IsAnyEnemyInRange
  (bind _asenemy_base (Utilities|Casting|CastToEnemyBase (.HitActor (|GetActorAndTraceEnd _outhit)))
    (:then
      (bind _result (Default|CheckWithinRange (Variables|Default|GetNozzle) _asenemy_base))
      (Variables|Default|SetIsAnyEnemyInRange _result))
    (:CastFailed
      (Variables|Default|SetIsAnyEnemyInRange false))))

(event EventPossessed
  (params (NewController :type Controller%20Object%20Reference))
  ;[1 1 1] Apply Crosshair
  (bind _asplayer_controller (Utilities|Casting|CastToPlayerController NewController))
  (bind _returnvalue (UserInterface|CreateWidget "/Game/Widget/Widget_Crosshair.Widget_Crosshair_C" _asplayer_controller))
  (bind _output_get (Variables|Default|SetCrosshairWidget _returnvalue))
  (Variables|/Game/Widget/Widget_Crosshair.Widget_Crosshair_C|SetCharacter _output_get self)
  (UserInterface|Viewport|AddtoPlayerScreen _output_get 300)
  (CallFunction|SetupSwitchNozzleWidget)
  ;[1 1 1] Apply Enemies Position Indicator Screen
  (bind _returnvalue_2 (UserInterface|CreateWidget "/Game/Widget/Widget_SplitScreen_PositionIndicatorScreen.Widget_SplitScreen_PositionIndicatorScreen_C" _asplayer_controller))
  (bind _output_get_2 (Variables|Default|SetEnemiesPositionIndicator _returnvalue_2))
  (UserInterface|Viewport|AddtoPlayerScreen _output_get_2))

(event Input|ActionEvents|InputActionPrimary_Fire
  (params (Key :type Key%20Structure))
  (bind _weapon (Variables|Default|GetWeapon))
  (bind _crosshairwidget (Variables|Default|GetCrosshairWidget))
  (:Pressed
    (Variables|Default|SetbUseControllerRotationYaw true)
    ;[1 1 1] Shoot
    (bind _rateoffire (Default|GetRateOfFire (Variables|/Game/Blueprints/Weapon/BP_Weapon.BP_Weapon_C|GetCurrentNozzle _weapon)))
    (Utilities|Time|SetTimerbyFunctionName _weapon "Primary" _rateoffire true)
    (Components|Activation|Activate (Variables|Default|GetPES_BubbleSucking) false)
    (Variables|Default|SetIsFiring true)
    (Animation|PlayAnimMontage "/Game/Meshes/Characters/Babooshka_Resized/AMontage_Sucking_Babooshka.AMontage_Sucking_Babooshka" 1.0 "Windup")
    (Default|PlayPrimarySound (Variables|Default|GetWeapon))
    (Default|StartShootEvent _crosshairwidget))
  (:Released
    (Variables|Default|SetbUseControllerRotationYaw false)
    ;[1 1 1] Stop Shooting
    (Utilities|Time|ClearTimerbyFunctionName _weapon "Primary")
    (Components|Activation|Deactivate (Variables|Default|GetPES_BubbleSucking))
    (Variables|Default|SetIsFiring false)
    (Animation|StopAnimMontage "/Game/Meshes/Characters/Babooshka_Resized/AMontage_Sucking_Babooshka.AMontage_Sucking_Babooshka")
    (Default|StopPrimarySound (Variables|Default|GetWeapon))
    (Default|StopShootEvent _crosshairwidget)))

(event Input|ActionEvents|InputActionSecondary_Fire
  (params (Key :type Key%20Structure))
  (bind _weapon (Variables|Default|GetWeapon))
  (:Pressed
    (if (not (Variables|Default|GetIsFiring))
      (Variables|Default|SetbUseControllerRotationYaw true)
      (Utilities|Time|SetTimerbyFunctionName _weapon "Secondary" 0.01 true)))
  (:Released
    (if (not (Variables|Default|GetIsFiring))
      (Variables|Default|SetbUseControllerRotationYaw false)
      (Utilities|Time|ClearTimerbyFunctionName _weapon "Secondary"))))

(event Input|ActionEvents|InputActionPreviousNozzle
  (params (Key :type Key%20Structure))
  (:Pressed
    (if (Variables|Default|GetIsInUI)
      (bind _shopinventorywidget (Variables|Default|GetShopInventoryWidget)
        (:then
          (Default|PreviousItemPressed _shopinventorywidget))
        (:else))
      (else
        (CallFunction|GotoNozzleIndex (- (Variables|Default|GetCurrentNozzleIndex) 1))))))

(event Input|ActionEvents|InputActionNextNozzle
  (params (Key :type Key%20Structure))
  (:Pressed
    (if (Variables|Default|GetIsInUI)
      (bind _shopinventorywidget (Variables|Default|GetShopInventoryWidget)
        (:then
          (Default|NextItemPressed _shopinventorywidget))
        (:else))
      (else
        (CallFunction|GotoNozzleIndex (+ (Variables|Default|GetCurrentNozzleIndex) 1))))))

(event Input|ActionEvents|InputActionInteract
  (params (Key :type Key%20Structure))
  (:Pressed
    (if (Variables|Default|GetIsInUI)
      (bind _shopinventorywidget (Variables|Default|GetShopInventoryWidget)
        (:then
          (Default|RepairBasePressed _shopinventorywidget))
        (:else))
      (else
        (Default|InteractedbyPlayer (Variables|Default|GetCurrentInteractable) self)))))

(event Input|ActionEvents|InputActionConfirm
  (params (Key :type Key%20Structure))
  (:Pressed
    (bind _shopinventorywidget (Variables|Default|GetShopInventoryWidget)
      (:then
        (Default|BuyButtonPressed _shopinventorywidget))
      (:else))))

(event Input|ActionEvents|InputActionExit
  (params (Key :type Key%20Structure))
  (:Pressed
    (bind _shopinventorywidget (Variables|Default|GetShopInventoryWidget)
      (:then
        (Default|ExitWindowPressed _shopinventorywidget))
      (:else))))

(fn ConstructionScript)

(fn InitWeapon
  (bind _self self)
  (bind _startingnozzle (Variables|Default|GetStartingNozzle))
  (bind _returnvalue (Game|SpawnActorfromClass "/Game/Blueprints/Weapon/BP_Weapon.BP_Weapon_C" (Math|Transform|MakeTransform "0, 0, 0" "0, 0, 0" "0.300000,0.300000,0.300000") "AlwaysSpawn" self 0))
  (bind _output_get (Variables|Default|SetWeapon _returnvalue))
  (Actor|SetOwner _returnvalue _self)
  (Variables|/Game/Blueprints/Weapon/BP_Weapon.BP_Weapon_C|SetCharacter _returnvalue _self)
  (Transformation|AttachComponentToComponent _returnvalue (Variables|Character|GetMesh) (Utilities|Name|MakeLiteralName "weapon_r") "KeepRelative" "KeepRelative" "KeepRelative" true)
  (bind _returnvalue_2 (Game|SpawnActorfromClass (Variables|/Game/Blueprints/Weapon/PDA_Nozzle.PDA_Nozzle_C|GetNozzleClass _startingnozzle) (Math|Transform|MakeTransform "0, 0, 0") "AlwaysSpawn" _returnvalue 0))
  (Default|InitNozzle _output_get _returnvalue_2 _startingnozzle)
  (Utilities|Array|AddUnique (Variables|Default|GetNozzleList) _startingnozzle)
  (Utilities|Map|Add (Variables|Default|GetNozzleToLevelList) _startingnozzle 0)
  (Default|SetNozzleProperties _returnvalue _startingnozzle)
  (Variables|/Game/Blueprints/Weapon/BP_NozzleBase.BP_NozzleBase_C|SetCharacter _returnvalue_2 self)
  (Variables|Default|SetNozzle _returnvalue_2)
  (Transformation|AttachComponentToComponent _returnvalue_2 (Variables|/Game/Blueprints/Weapon/BP_Weapon.BP_Weapon_C|GetWeaponMesh _returnvalue) "nozzle" "KeepRelative" "KeepRelative" "KeepRelative" true))

(fn InitVacuumBag
  (bind _returnvalue (Game|SpawnActorfromClass "/Game/Blueprints/Weapon/BP_VacuumBag.BP_VacuumBag_C" (Math|Transform|MakeTransform "0, 0, 0" "0, 0, 0" "0.400000,0.400000,0.400000") "AlwaysSpawn" self 0))
  (bind _output_get (Variables|Default|SetBag _returnvalue))
  (Actor|SetOwner _output_get self)
  (Transformation|AttachComponentToComponent _output_get (Variables|Character|GetMesh) "Back" "KeepRelative" "KeepRelative" "KeepRelative" true))

(fn KilledEnemy
  (bind _matterout (Default|ProcessMatter (Variables|Default|GetWeapon) 0.0))
  (Default|ChangeMatterValueby (Variables|Default|GetBag) _matterout))

(fn TransferNozzle
  (params (IncomingNozzle :type PDA%20Nozzle%20Object%20Reference))
  (bind _nozzletolevellist (Variables|Default|GetNozzleToLevelList))
  (bind _nozzlelist (Variables|Default|GetNozzleList))
  (bind _nozzlelist_2 (Variables|Default|GetNozzleList))
  (bind _returnvalue (Utilities|Array|FindItem _nozzlelist_2 IncomingNozzle))
  (bind _value (Utilities|Map|Find _nozzletolevellist IncomingNozzle))
  (if (Utilities|Array|ContainsItem _nozzlelist IncomingNozzle)
    ;[1 1 1] Adds 1 level to Nozzle
    (if (Utilities|Map|Contains _nozzletolevellist IncomingNozzle)
      (Utilities|Map|Add _nozzletolevellist IncomingNozzle (+ _value 1))
      (CallFunction|GotoNozzleIndex _returnvalue)
      (Default|SetNozzleProperties (Variables|Default|GetWeapon) IncomingNozzle _value)
      (else
        ;[1 1 1] Insert Nozzle
        (Utilities|Map|Add _nozzletolevellist IncomingNozzle 0 :!label _label)
        (CallFunction|GotoNozzleIndex _returnvalue)
        (Default|SetNozzleProperties (Variables|Default|GetWeapon) IncomingNozzle)))
    (else
      (Utilities|Array|AddUnique _nozzlelist IncomingNozzle)
      (goto _label))))

(fn SwitchNozzle
  (params (NewNozzle :type PDA%20Nozzle%20Object%20Reference))
  (bind _nozzletolevellist (Variables|Default|GetNozzleToLevelList))
  (bind (_value _returnvalue) (Utilities|Map|Find _nozzletolevellist NewNozzle))
  (if _returnvalue
    (Default|SetNozzleProperties (Variables|Default|GetWeapon) NewNozzle _value)))

(fn SetupSwitchNozzleWidget
  (bind _asplayer_controller (Utilities|Casting|CastToPlayerController (Pawn|GetController self)))
  (bind _returnvalue (UserInterface|CreateWidget "/Game/Widget/WBP_NozzleSwitch.WBP_NozzleSwitch_C" _asplayer_controller))
  (bind _output_get (Variables|Default|SetNozzleSwitchWidget _returnvalue))
  (Variables|/Game/Widget/WBP_NozzleSwitch.WBP_NozzleSwitch_C|SetPlayer _output_get self)
  (UserInterface|Viewport|AddtoPlayerScreen _returnvalue 200))

(fn GotoNozzleIndex
  (params (ToIndex :type Integer))
  (bind _nozzlelist (Variables|Default|GetNozzleList))
  (bind _returnvalue (Utilities|Array|Length _nozzlelist))
  (bind _output_get (LocalVariables|SetOldIndex (Variables|Default|GetCurrentNozzleIndex)))
  (if (>= ToIndex _returnvalue)
    (LocalVariables|SetNewIndex 0)
    (elif (< ToIndex 0)
      (LocalVariables|SetNewIndex (- _returnvalue 1))
      (else
        (bind _output_get_2 (LocalVariables|SetNewIndex ToIndex)))))
  (CallFunction|SwitchNozzle (Utilities|Array|Get(acopy) _nozzlelist (LocalVariables|GetNewIndex)))
  (Variables|Default|SetCurrentNozzleIndex _output_get_2)
  (Default|CallOnNozzleIndexChange _output_get))

(fn PushedBack
  (params (Direction :type Vector) (Intensity :type Float%20%28single-precision%29))
  (bind _returnvalue (* Direction Intensity))
  (Physics|AddImpulse (Variables|Character|GetCharacterMovement) _returnvalue true)
  (Effects|SpawnEmitteratLocation "/Game/ParticleEffects/PES_Pushed.PES_Pushed" (Transformation|GetActorLocation) (Math|Conversions|RotationFromXVector _returnvalue)))

(fn DealingDamage
  (Variables|Default|SetIsDealingDamage true)
  (Utilities|Time|SetTimerbyFunctionName 0 "SetFalseDealingDamage" 0.5))

(fn SetFalseDealingDamage
  (Variables|Default|SetIsDealingDamage false))