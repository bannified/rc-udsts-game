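; Game mode base that runs a wave-based game as a state machine of spawned state objects.
; StartGame stores the level data asset and enters a setup state; NextWave spawns one for each following wave, printing a win message when none remain.
; ChangeToState runs stop, exit, enter and start hooks and broadcasts the change, while Tick updates the current state.
; Spawned enemies are counted through their destroyed events.
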(event Custom|OnStateChanged_Event
  (params (OldState :type Game%20Mode%20State%20Object%20Reference) (NewState :type Game%20Mode%20State%20Object%20Reference)))

(event Custom|EnemyDestroyed
  (params (EnemyDestroyed :type Actor%20Object%20Reference))
  (Math|Integer|DecrementInt (Variables|Default|GetEnemiesInGame)
    (:%20%20
      (Development|PrintString (Utilities|String|Append "UDSGameModeBase: " (Utilities|GetDisplayName EnemyDestroyed) " destroyed."))
      (Game|UnbindEventfromOnDestroyed EnemyDestroyed (EventDispatchers|CreateEvent :!event Custom|EnemyDestroyed)))))

(event EventBeginPlay)

(event EventTick
  (params (DeltaSeconds :type Float%20%28single-precision%29))
  (bind _currentstate (Variables|Default|GetCurrentState))
  (Utilities|IsValid _currentstate
    (:Is%20Valid
      (bind _asudsgame_mode_base (Utilities|Casting|CastToUDSGameModeBase (Game|GetGameMode)))
      (Class|GameModeState|OnStateTick _currentstate _asudsgame_mode_base DeltaSeconds))))

(fn ConstructionScript)

(fn NextWave
  (bind _currentwaveindex (Variables|Default|GetCurrentWaveIndex))
  (bind _mapleveldataasset (Variables|Default|GetMapLevelDataAsset))
  (bind _waves (Variables|/Script/UDSTS.LevelDataAsset|GetWaves _mapleveldataasset))
  (Math|Integer|IncrementInt (Variables|Default|GetCurrentWaveIndex)
    (:%20%20
      (if (< _currentwaveindex (Utilities|Array|Length _waves))
        ;[1 1 1] create next wave's setup
        (bind _returnvalue (Game|SpawnActorfromClass "/Game/GameModePrototype/GameModeStatesPrototype/BP_GMS_SetupState.BP_GMS_SetupState_C" (Math|Transform|MakeTransform "0, 0, 0") "AlwaysSpawn" 0 0))
        (Default|Init _returnvalue (Utilities|Array|Get(acopy) _waves _currentwaveindex))
        (CallFunction|ChangetoState _returnvalue)
        (else
          (Development|PrintString "No more levels left, win!"))))))

(fn StartGame
  (params (LevelData :type Level%20Data%20Asset%20Object%20Reference) (Game%20Mode :type BP%20UDS%20Game%20Mode%20Base%20Object%20Reference))
  (bind _output_get (Variables|Default|SetMapLevelDataAsset LevelData))
  (bind _returnvalue (Game|SpawnActorfromClass "/Game/GameModePrototype/GameModeStatesPrototype/BP_GMS_SetupState.BP_GMS_SetupState_C" (Math|Transform|MakeTransform "0, 0, 0") "AlwaysSpawn" self 0))
  (Default|Init _returnvalue (Utilities|Array|Get(acopy) (Variables|/Script/UDSTS.LevelDataAsset|GetWaves _output_get) (Variables|Default|GetCurrentSpawnUnitIndex)))
  (CallFunction|ChangetoState Game%20Mode _returnvalue))

(fn ChangetoState
  (params (NewState :type Game%20Mode%20State%20Object%20Reference))
  (bind _self self)
  (Utilities|IsValid (Variables|Default|GetCurrentState)
    (:Is%20Valid
      (bind _output_get (LocalVariables|SetOldState (Variables|Default|GetCurrentState)))
      (Class|GameModeState|OnStateStop (Variables|Default|GetCurrentState) _self)
      (Class|GameModeState|OnStateExit (Variables|Default|GetCurrentState) _self))
    (:Is%20Not%20Valid
      _))
  (bind _output_get_2 (Variables|Default|SetCurrentState NewState))
  (Class|GameModeState|OnStateEnter _output_get_2 _self)
  (Class|GameModeState|OnStateStart _output_get_2 _self)
  (CallFunction|OnStateChangedEvent _output_get _output_get_2))

(fn HandleEnemySpawn
  (params (SpawnedEnemy :type Actor%20Object%20Reference))
  (Game|BindEventtoOnDestroyed SpawnedEnemy (EventDispatchers|CreateEvent :!event Custom|EnemyDestroyed))
  (Math|Integer|IncrementInt (Variables|Default|GetEnemiesInGame)))