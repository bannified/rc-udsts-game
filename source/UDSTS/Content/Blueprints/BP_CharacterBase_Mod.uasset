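; Character base Blueprint that initializes health and equips a modular weapon with an interchangeable nozzle.
; On BeginPlay it sets up BPCHealth, spawns BP_Weapon onto the mesh's weapon_r socket, then assigns and attaches a blow nozzle to the weapon.
; Fire inputs start and clear looping timers that call the weapon's Primary and Secondary functions by name, with primary paced by the nozzle's rate of fire.
; InitWeapon is an empty stub.
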(event EventBeginPlay
  (Default|InitHealth (Variables|Default|GetBPC_Health) (Variables|Default|GetStartingHealth))
  (bind _returnvalue (Game|SpawnActorfromClass "/Game/Blueprints/Weapon/BP_Weapon.BP_Weapon_C" (Math|Transform|MakeTransform "0, 0, 0") "Undefined" 0 0))
  (bind _output_get (Variables|Default|SetCurrentWeapon _returnvalue))
  (Transformation|AttachComponentToComponent _output_get (Variables|Character|GetMesh) "weapon_r" "KeepRelative" "KeepRelative" "KeepRelative" true)
  (bind _returnvalue_2 (Game|SpawnActorfromClass "/Game/Blueprints/Weapon/BP_NozzleBlow.BP_NozzleBlow_C" (Math|Transform|MakeTransform "0, 0, 0") "Undefined" 0 0))
  (Default|SetNozzle (Variables|Default|GetCurrentWeapon) _returnvalue_2)
  (Transformation|AttachComponentToComponent _returnvalue_2 (Variables|/Game/Blueprints/Weapon/BP_Weapon.BP_Weapon_C|GetWeaponMesh _output_get) "" "KeepRelative" "KeepRelative" "KeepRelative" true))

(event Collision|EventActorBeginOverlap
  (params (OtherActor :type Actor%20Object%20Reference)))

(event EventTick
  (params (DeltaSeconds :type Float%20%28single-precision%29)))

(event Input|ActionEvents|InputActionPrimary_Fire
  (params (Key :type Key%20Structure))
  (bind _currentweapon (Variables|Default|GetCurrentWeapon))
  (:Pressed
    (Utilities|Time|SetTimerbyFunctionName _currentweapon "Primary" (Variables|/Game/Blueprints/Weapon/BP_NozzleBase.BP_NozzleBase_C|GetRateOfFire (Variables|/Game/Blueprints/Weapon/BP_Weapon.BP_Weapon_C|GetCurrentNozzle _currentweapon)) true))
  (:Released
    (Utilities|Time|ClearTimerbyFunctionName _currentweapon "Primary")))

(event Input|ActionEvents|InputActionSecondary_Fire
  (params (Key :type Key%20Structure))
  (bind _currentweapon (Variables|Default|GetCurrentWeapon))
  (:Pressed
    (Utilities|Time|SetTimerbyFunctionName _currentweapon "Secondary" 0.01 true))
  (:Released
    (Utilities|Time|ClearTimerbyFunctionName _currentweapon "Secondary")))

(fn ConstructionScript)

(fn InitWeapon)