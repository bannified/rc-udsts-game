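; Split-screen variant of the Babooshka character that gives the possessing player their own HUD widget.
; On possession by a player controller, it creates a WBP_Player owned by that controller, passes itself as the widget's Character and adds it to that player's screen at a high Z-order.
; BeginPlay and construction only call the parent.
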(event EventBeginPlay
  (|CallParentFunction))

(event Collision|EventActorBeginOverlap
  (params (OtherActor :type Actor%20Object%20Reference))
  (|CallParentFunction OtherActor) ; This node is disabled and will not be called.\nDrag off pins to build functionality.
)

(event EventTick
  (params (DeltaSeconds :type Float%20%28single-precision%29))
  (|CallParentFunction DeltaSeconds) ; This node is disabled and will not be called.\nDrag off pins to build functionality.
)

(event EventPossessed
  (params (NewController :type Controller%20Object%20Reference))
  (bind _asplayer_controller (Utilities|Casting|CastToPlayerController NewController))
  (bind _returnvalue (UserInterface|CreateWidget "/Game/Widget/WBP_Player.WBP_Player_C" _asplayer_controller))
  (Variables|/Game/Widget/WBP_Player.WBP_Player_C|SetCharacter _returnvalue self)
  (UserInterface|Viewport|AddtoPlayerScreen _returnvalue 99))

(fn ConstructionScript
  (|CallParentFunction))