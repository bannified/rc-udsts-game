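; Player character Babooshka, armed with a vacuum weapon and back-mounted bag that are spawned and attached to mesh sockets on BeginPlay.
; Fire inputs loop the weapon's Primary and Secondary functions by timer, with primary adding sucking montage, particles and audio.
; Tick pitches weapon colliders to control rotation, and kills feed processed matter into the bag.
; A nozzle-to-level map tracks pickups, levels up duplicates and supplies weapon properties on switching.
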(event Custom|OnBoostActivated_Event_0
  (params (Charater :type Character%20Base%20Object%20Reference))
  (Effects|SpawnEmitterAttached (Variables|Default|GetBoosterParticleSystem) (Variables|/Game/Blueprints/Weapon/BP_VacuumBag.BP_VacuumBag_C|GetVacuumBag (Variables|Default|GetBag)) (Variables|Default|GetBoosterEndSocketName) "0, 0, 0" "0, 0, 0" (Variables|Default|GetBoosterParticleScale) "KeepRelativeOffset" true "AutoRelease"))

(event EventBeginPlay
  (CallFunction|InitWeapon)
  (CallFunction|InitVacuumBag)
  (EventDispatchers|AssignOnBoostActivated (delegate Custom|OnBoostActivated_Event_0)))

(event Collision|EventActorBeginOverlap
  (params (OtherActor :type Actor%20Object%20Reference)))

(event EventTick
  (params (DeltaSeconds :type Float%20%28single-precision%29))
  (bind _capsulecomponent (Variables|Default|GetCapsuleComponent))
  (bind _returnvalue (Transformation|GetWorldRotation _capsulecomponent))
  ;[1 1 1] Set Colliders' Pitch
  (Transformation|SetWorldRotation (Variables|Default|GetWeaponColliders) (Math|Rotator|MakeRotator (.roll _returnvalue) (.pitch (Pawn|GetControlRotation :!class /Script/Engine.Pawn)) (.yaw _returnvalue)) false false))

(event Input|ActionEvents|InputActionPrimary_Fire
  (params (Key :type Key%20Structure))
  (bind _weapon (Variables|Default|GetWeapon))
  (:Pressed
    (Variables|Default|SetbUseControllerRotationYaw true)
    ;[1 1 1] Shoot
    (bind _rateoffire (Default|GetRateOfFire (Variables|/Game/Blueprints/Weapon/BP_Weapon.BP_Weapon_C|GetCurrentNozzle _weapon)))
    (Utilities|Time|SetTimerbyFunctionName _weapon "Primary" _rateoffire true)
    (Components|Activation|Activate (Variables|Default|GetPES_BubbleSucking) false)
    (Variables|Default|SetIsFiring true)
    (Animation|PlayAnimMontage "/Game/Meshes/Characters/Babooshka_Resized/AMontage_Sucking_Babooshka.AMontage_Sucking_Babooshka" 1.0 "Windup")
    (Audio|Components|Audio|Play (Variables|Default|GetAudio) 0.0))
  (:Released
    (Variables|Default|SetbUseControllerRotationYaw false)
    ;[1 1 1] Stop Shooting
    (Utilities|Time|ClearTimerbyFunctionName _weapon "Primary")
    (Components|Activation|Deactivate (Variables|Default|GetPES_BubbleSucking))
    (Variables|Default|SetIsFiring false)
    (Animation|StopAnimMontage "/Game/Meshes/Characters/Babooshka_Resized/AMontage_Sucking_Babooshka.AMontage_Sucking_Babooshka")
    (Audio|Components|Audio|Stop (Variables|Default|GetAudio))))

(event Input|ActionEvents|InputActionSecondary_Fire
  (params (Key :type Key%20Structure))
  (bind _weapon (Variables|Default|GetWeapon))
  (:Pressed
    (Variables|Default|SetbUseControllerRotationYaw true)
    (Utilities|Time|SetTimerbyFunctionName _weapon "Secondary" 0.01 true))
  (:Released
    (Variables|Default|SetbUseControllerRotationYaw false)
    (Utilities|Time|ClearTimerbyFunctionName _weapon "Secondary")))

(fn ConstructionScript)

(fn InitWeapon
  (bind _self self)
  (bind _startingnozzle (Variables|Default|GetStartingNozzle))
  (bind _returnvalue (Game|SpawnActorfromClass "/Game/Blueprints/Weapon/BP_Weapon.BP_Weapon_C" (Math|Transform|MakeTransform "0, 0, 0" "0, 0, 0" "0.300000,0.300000,0.300000") "AlwaysSpawn" self 0))
  (bind _output_get (Variables|Default|SetWeapon _returnvalue))
  (Actor|SetOwner _returnvalue _self)
  (Variables|/Game/Blueprints/Weapon/BP_Weapon.BP_Weapon_C|SetCharacter _returnvalue _self)
  (Transformation|AttachComponentToComponent _returnvalue (Variables|Character|GetMesh) (Utilities|Name|MakeLiteralName "weapon_r") "KeepRelative" "KeepRelative" "KeepRelative" true)
  (bind _returnvalue_2 (Game|SpawnActorfromClass (Variables|/Game/Blueprints/Weapon/PDA_Nozzle.PDA_Nozzle_C|GetNozzleClass _startingnozzle) (Math|Transform|MakeTransform "0, 0, 0") "AlwaysSpawn" _returnvalue 0))
  (Default|InitNozzle _output_get _returnvalue_2 _startingnozzle)
  (Utilities|Array|AddUnique (Variables|Default|GetNozzleList) _startingnozzle)
  (Utilities|Map|Add (Variables|Default|GetNozzleToLevelList) _startingnozzle 0)
  (Default|SetNozzleProperties _returnvalue _startingnozzle)
  (Variables|/Game/Blueprints/Weapon/BP_NozzleBase.BP_NozzleBase_C|SetCharacter _returnvalue_2 self)
  (Variables|Default|SetNozzle _returnvalue_2)
  (Transformation|AttachComponentToComponent _returnvalue_2 (Variables|/Game/Blueprints/Weapon/BP_Weapon.BP_Weapon_C|GetWeaponMesh _returnvalue) "nozzle" "KeepRelative" "KeepRelative" "KeepRelative" true))

(fn InitVacuumBag
  (bind _returnvalue (Game|SpawnActorfromClass "/Game/Blueprints/Weapon/BP_VacuumBag.BP_VacuumBag_C" (Math|Transform|MakeTransform "0, 0, 0" "0, 0, 0" "0.400000,0.400000,0.400000") "AlwaysSpawn" self 0))
  (bind _output_get (Variables|Default|SetBag _returnvalue))
  (Actor|SetOwner _output_get self)
  (Transformation|AttachComponentToComponent _output_get (Variables|Character|GetMesh) "Back" "KeepRelative" "KeepRelative" "KeepRelative" true))

(fn KilledEnemy
  (bind _matterout (Default|ProcessMatter (Variables|Default|GetWeapon) 0.0))
  (Default|ChangeMatterValueby (Variables|Default|GetBag) _matterout))

(fn TransferNozzle
  (params (IncomingNozzle :type PDA%20Nozzle%20Object%20Reference))
  (bind _nozzletolevellist (Variables|Default|GetNozzleToLevelList))
  (bind _nozzlelist (Variables|Default|GetNozzleList))
  (bind _value (Utilities|Map|Find _nozzletolevellist IncomingNozzle))
  (bind _returnvalue (+ _value 1))
  (if (Utilities|Array|ContainsItem _nozzlelist IncomingNozzle)
    ;[1 1 1] Adds 1 level to Nozzle
    (if (Utilities|Map|Contains _nozzletolevellist IncomingNozzle)
      (Utilities|Map|Add _nozzletolevellist IncomingNozzle _returnvalue)
      (Default|SetNozzleProperties (Variables|Default|GetWeapon) IncomingNozzle _returnvalue)
      (else
        ;[1 1 1] Insert Nozzle
        (Utilities|Map|Add _nozzletolevellist IncomingNozzle 0 :!label _label)
        (Default|SetNozzleProperties (Variables|Default|GetWeapon) IncomingNozzle)))
    (else
      (Utilities|Array|AddUnique _nozzlelist IncomingNozzle)
      (goto _label))))

(fn SwitchNozzle
  (params (NewNozzle :type PDA%20Nozzle%20Object%20Reference))
  (bind _nozzletolevellist (Variables|Default|GetNozzleToLevelList))
  (bind (_value _returnvalue) (Utilities|Map|Find _nozzletolevellist NewNozzle))
  (if _returnvalue
    (Default|SetNozzleProperties (Variables|Default|GetWeapon) NewNozzle _value)))