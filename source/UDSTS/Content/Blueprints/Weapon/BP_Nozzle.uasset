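; BP_Nozzle is a weapon Blueprint that provides a secondary attack which shoves a chosen target and damages enemies.
; Secondary checks a readiness flag, clears it, starts a named-function cooldown timer that restores it, then calls ActivateSecondary.
; ActivateSecondary applies a power-scaled impulse along the player camera's forward vector to the target's primitive component, then deals damage only if the target is a BP_Enemy.
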(event EventBeginPlay)

(event Collision|EventActorBeginOverlap
  (params (OtherActor :type Actor%20Object%20Reference)))

(event EventTick
  (params (DeltaSeconds :type Float%20%28single-precision%29)))

(fn ConstructionScript)

(fn SecondaryReady
  (Variables|Default|SetIsSecondaryReady true))

(fn ActivateSecondary
  (params (Object :type Actor%20Object%20Reference))
  (Physics|AddImpulse (Actor|GetComponentbyClass Object "/Script/Engine.PrimitiveComponent") (* (Transformation|GetActorForwardVector (Game|GetPlayerCameraManager 0)) (* (Variables|Default|GetSecondaryPower) 1e+05)) "None" false)
  (bind _asbp_enemy (Utilities|Casting|CastToBP_Enemy Object))
  (Default|TakeDamage _asbp_enemy (Variables|Default|GetSecondaryDamage)))

(fn Secondary
  (params (Chosen%20Target :type Actor%20Object%20Reference))
  (if (Variables|Default|GetIsSecondaryReady)
    (Variables|Default|SetIsSecondaryReady false)
    (Utilities|Time|SetTimerbyFunctionName 0 "SecondaryReady" (Variables|Default|GetSecondaryCooldown))
    (CallFunction|ActivateSecondary Chosen%20Target))
  (return false))