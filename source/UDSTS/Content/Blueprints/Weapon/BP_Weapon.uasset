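; BP_Weapon is a weapon actor that delegates its behavior to an interchangeable nozzle held in CurrentNozzle.
; Primary, Secondary and UpgradeWeapon forward to the nozzle, while ProcessMatter scales incoming matter by the nozzle's conversion value.
; InitNozzle assigns a nozzle, sets its owner to the weapon's owner and applies its data and mesh; SetNozzleProperties swaps data and mesh on the current nozzle and resets its level.
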(event EventBeginPlay)

(event Collision|EventActorBeginOverlap
  (params (OtherActor :type Actor%20Object%20Reference)))

(event EventTick
  (params (DeltaSeconds :type Float%20%28single-precision%29)))

(fn ConstructionScript)

(fn Primary
  (Default|Primary (Variables|Default|GetCurrentNozzle)))

(fn Secondary
  (Default|Secondary (Variables|Default|GetCurrentNozzle)))

(fn SetNozzleProperties
  (params (NewNozzleData :type PDA%20Nozzle%20Object%20Reference))
  (bind _currentnozzle (Variables|Default|GetCurrentNozzle))
  (Variables|/Game/Blueprints/Weapon/BP_NozzleBase.BP_NozzleBase_C|SetNozzleData _currentnozzle NewNozzleData)
  (Components|StaticMesh|SetStaticMesh (Variables|/Game/Blueprints/Weapon/BP_NozzleBase.BP_NozzleBase_C|GetNozzleMesh _currentnozzle) (Variables|/Game/Blueprints/Weapon/PDA_Nozzle.PDA_Nozzle_C|GetMeshModel NewNozzleData))
  (Variables|/Game/Blueprints/Weapon/BP_NozzleBase.BP_NozzleBase_C|SetLevel _currentnozzle 0))

(fn ProcessMatter
  (params (MatterIn :type Float%20%28single-precision%29))
  (bind _conversion (Default|GetConversion (Variables|Default|GetCurrentNozzle)))
  (return (* _conversion MatterIn)))

(fn UpgradeWeapon
  (Default|UpgradeNozzle (Variables|Default|GetCurrentNozzle)))

(fn InitNozzle
  (params (NewNozzle :type BP%20Nozzle%20Base%20Object%20Reference) (NewStats :type PDA%20Nozzle%20Object%20Reference))
  (bind _output_get (Variables|Default|SetCurrentNozzle NewNozzle))
  (Actor|SetOwner _output_get (Components|GetOwner))
  (Variables|/Game/Blueprints/Weapon/BP_NozzleBase.BP_NozzleBase_C|SetNozzleData _output_get NewStats)
  (Components|StaticMesh|SetStaticMesh (Variables|/Game/Blueprints/Weapon/BP_NozzleBase.BP_NozzleBase_C|GetNozzleMesh _output_get) (Variables|/Game/Blueprints/Weapon/PDA_Nozzle.PDA_Nozzle_C|GetMeshModel NewStats)))