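; Blow nozzle weapon whose secondary fire blasts enemies away and recoils the player.
; When off cooldown, Secondary restarts the timer, gathers EnemyBase actors overlapping the character's Cone, spawns particles at a nozzle socket and returns true.
; Each unobstructed target takes damage and a camera-forward impulse scaled by inverse distance through a power curve.
; Feedback launches the player opposite the cone's up vector, scaled by secondary power.
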(event EventBeginPlay)

(event Collision|EventActorBeginOverlap
  (params (OtherActor :type Actor%20Object%20Reference)))

(event EventTick
  (params (DeltaSeconds :type Float%20%28single-precision%29)))

(fn ConstructionScript)

(fn SecondaryReady
  (Variables|Default|SetIsSecondaryReady true))

(fn ActivateSecondary
  (params (Objects :type Actor%20Object%20Reference))
  (bind _result (CallFunction|CheckifPathObstructed Objects))
  (if (not _result)
    ;[1 1 1] Blow Enemy
    (bind _secondarypower (CallFunction|GetSecondaryPower))
    (Physics|AddImpulse (Actor|GetComponentbyClass Objects "/Script/Engine.PrimitiveComponent") (* (Transformation|GetActorForwardVector (Game|GetPlayerCameraManager 0)) (* _secondarypower 1e+05 (Math|Float|Power (* (+ (/ 1.0 (Transformation|GetDistanceTo Objects self)) 1.0) 1.2) 6.0))) "None" false)
    ;[1 1 1] Apply Damage
    (bind _secondarydamage (CallFunction|GetSecondaryDamage))
    (Game|Damage|ApplyDamage Objects _secondarydamage 0 (Variables|Default|GetCharacter))))

(fn Feedback
  (bind _secondarypower (CallFunction|GetSecondaryPower))
  (Physics|AddImpulse (Variables|/Script/Engine.Character|GetCharacterMovement (Game|GetPlayerCharacter 0)) (* (* (Math|Vector|GetUpVector (Variables|/Game/Blueprints/BP_Babooshka.BP_Babooshka_C|GetCone (Variables|Default|GetCharacter))) -1.0) (* _secondarypower 1e+03)) true))

(fn GetTargetSecondary
  (return (Collision|GetOverlappingActors (Variables|/Game/Blueprints/BP_Babooshka.BP_Babooshka_C|GetCone (Variables|Default|GetCharacter)) "/Script/UDSTS.EnemyBase" :!class /Script/Engine.PrimitiveComponent)))

(fn Secondary
  (bind _character (Variables|Default|GetCharacter))
  (bind _cone (Variables|/Game/Blueprints/BP_Babooshka.BP_Babooshka_C|GetCone _character))
  (bind _returnvalue (Transformation|GetWorldRotation _cone))
  (if (Variables|Default|GetIsSecondaryReady)
    (Variables|Default|SetIsSecondaryReady false)
    (bind _secondarycooldown (CallFunction|GetSecondaryCooldown))
    (Utilities|Time|SetTimerbyFunctionName 0 "SecondaryReady" _secondarycooldown)
    (bind _enemies (CallFunction|GetTargetSecondary))
    (for _array_element _enemies
      (CallFunction|ActivateSecondary _array_element))
    (CallFunction|Feedback)
    (Effects|SpawnEmitteratLocation (Variables|Default|GetSecondaryParticleSystem) (Transformation|GetSocketLocation (Variables|Default|GetNozzleMesh) (Variables|Default|GetSecondaryParticleSystemSocketName)) (Math|Rotator|MakeRotator (.roll _returnvalue) (+ (.pitch _returnvalue) 9e+01) (.yaw _returnvalue)) (Variables|Default|GetSecondaryParticleScale) true "AutoRelease")
    (return true)
    (else
      (return false))))