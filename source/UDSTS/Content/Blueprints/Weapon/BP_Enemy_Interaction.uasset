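; BP_Enemy_Interaction is an enemy Blueprint with health, movement speed and a Matter value, all set on BeginPlay.
; It initializes its BPCHealth component and binds that component's death event to a handler that prints a debug message and destroys the actor.
; Tick is empty and overlap is disabled, while damage and health-printing nodes are left unconnected.
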(event Custom|DeathEvent
  (Development|PrintString "Enemy ees ded")
  (Actor|DestroyActor))

(event EventBeginPlay
  (bind _bpc_health (Variables|Default|GetBPC_Health))
  (|CallParentFunction)
  (Default|InitHealth _bpc_health 1e+02)
  (EventDispatchers|BindEventtoDeathEvent _bpc_health (delegate Custom|DeathEvent))
  (Variables|Default|SetMovementSpeed 1e+02)
  (Variables|Default|SetMatter 1e+02))

(event Collision|EventActorBeginOverlap
  (params (OtherActor :type Actor%20Object%20Reference))
  (|CallParentFunction OtherActor) ; This node is disabled and will not be called.\nDrag off pins to build functionality.
)

(event EventTick
  (params (DeltaSeconds :type Float%20%28single-precision%29)))

(fn ConstructionScript
  (|CallParentFunction))