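; Blow nozzle weapon whose secondary fire blasts enemies away from the player, gated by a timer-based cooldown.
; Secondary gathers EnemyBase actors overlapping the character's Cone, skips obstructed ones, then applies a camera-forward impulse that strengthens with proximity, plus damage to BP_Enemy targets.
; Each shot also recoils the player opposite the owner's forward vector and spawns a particle burst at the nozzle socket.
; An alternative line-trace targeting function exists but is not called here.
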(event EventBeginPlay)

(event Collision|EventActorBeginOverlap
  (params (OtherActor :type Actor%20Object%20Reference)))

(event EventTick
  (params (DeltaSeconds :type Float%20%28single-precision%29)))

(fn ConstructionScript)

(fn SecondaryReady
  (Variables|Default|SetIsSecondaryReady true))

(fn ActivateSecondary
  (params (Objects :type Actor%20Object%20Reference))
  (bind _result (CallFunction|CheckifPathObstructed Objects))
  (if (not _result)
    ;[1 1 1] Blow Enemy
    (bind _secondarypower (CallFunction|GetSecondaryPower))
    (Physics|AddImpulse (Actor|GetComponentbyClass Objects "/Script/Engine.PrimitiveComponent") (* (Transformation|GetActorForwardVector (Game|GetPlayerCameraManager 0)) (* _secondarypower 1e+05 (Math|Float|Power (* (+ (/ 1.0 (Transformation|GetDistanceTo Objects self)) 1.0) 1.2) 6.0))) "None" false)
    ;[1 1 1] Apply Damage
    (bind _asbp_enemy (Utilities|Casting|CastToBP_Enemy Objects))
    (bind _secondarydamage (CallFunction|GetSecondaryDamage))
    (Default|TakeDamage _asbp_enemy _secondarydamage (Components|GetOwner))))

(fn Feedback
  (bind _secondarypower (CallFunction|GetSecondaryPower))
  (Physics|AddImpulse (Variables|/Script/Engine.Character|GetCharacterMovement (Game|GetPlayerCharacter 0)) (* (* (Transformation|GetActorForwardVector (Components|GetOwner)) -1.0) (* _secondarypower 1e+03)) true))

(fn GetTargetSecondary
  (return (Collision|GetOverlappingActors (Variables|/Game/Blueprints/BP_Babooshka.BP_Babooshka_C|GetCone (Variables|Default|GetCharacter)) "/Script/UDSTS.EnemyBase" :!class /Script/Engine.PrimitiveComponent)))

(fn Secondary
  (if (Variables|Default|GetIsSecondaryReady)
    (Variables|Default|SetIsSecondaryReady false)
    (bind _secondarycooldown (CallFunction|GetSecondaryCooldown))
    (Utilities|Time|SetTimerbyFunctionName 0 "SecondaryReady" _secondarycooldown)
    (bind _enemies (CallFunction|GetTargetSecondary))
    (for _array_element _enemies
      (CallFunction|ActivateSecondary _array_element))
    (CallFunction|Feedback)
    (Effects|SpawnEmitteratLocation (Variables|Default|GetSecondaryParticleSystem) (Transformation|GetSocketLocation (Variables|Default|GetNozzleMesh) (Variables|Default|GetSecondaryParticleSystemSocketName)) (Transformation|GetWorldRotation (Variables|/Game/Blueprints/BP_Babooshka.BP_Babooshka_C|GetCone (Variables|Default|GetCharacter))) (Variables|Default|GetSecondaryParticleScale) true "AutoRelease")
    (return true)
    (else
      (return false))))

(fn GetTargetSecondary0
  (bind _returnvalue (Game|GetPlayerCameraManager 0))
  (bind _returnvalue_2 (Transformation|GetActorForwardVector _returnvalue))
  (bind _returnvalue_3 (* _returnvalue_2 10000))
  (Collision|MultiLineTraceByChannel (+ (Transformation|GetActorLocation _returnvalue) _returnvalue_3) _returnvalue_3 "TraceTypeQuery1" false 0 "None")
  (for _array_element 0
    (bind _asbp_enemy (Utilities|Casting|CastToBP_Enemy (.hitactor _array_element)))
    (Utilities|Array|Add (LocalVariables|GetEnemiesAffected) _asbp_enemy))
  (return (LocalVariables|GetEnemiesAffected)))