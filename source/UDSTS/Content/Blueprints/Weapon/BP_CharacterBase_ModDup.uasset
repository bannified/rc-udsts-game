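; Player character base for a vacuum-weapon game, spawning a weapon with a blow nozzle and a vacuum bag on BeginPlay.
; Fire inputs loop the weapon's Primary (at nozzle fire rate) and Secondary functions through named timers, and H upgrades the weapon.
; KilledEnemy feeds matter through the weapon into the bag, and PushedBack applies an impulse.
; The bag's attach node is unwired, so it spawns unattached.
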(event EventBeginPlay
  (bind _mesh (Variables|Character|GetMesh))
  (Default|InitHealth (Variables|Default|GetBPC_Health) (Variables|Default|GetStartingHealth))
  (CallFunction|InitWeapon _mesh "weapon_r")
  (CallFunction|InitVacuumBag _mesh "None"))

(event Collision|EventActorBeginOverlap
  (params (OtherActor :type Actor%20Object%20Reference)))

(event EventTick
  (params (DeltaSeconds :type Float%20%28single-precision%29)))

(event Input|ActionEvents|InputActionPrimary_Fire
  (params (Key :type Key%20Structure))
  (bind _currentweapon (Variables|Default|GetCurrentWeapon))
  (:Pressed
    (bind _rateoffire (Default|GetRateOfFire (Variables|/Game/Blueprints/Weapon/BP_Weapon.BP_Weapon_C|GetCurrentNozzle _currentweapon)))
    (Utilities|Time|SetTimerbyFunctionName _currentweapon "Primary" _rateoffire true))
  (:Released
    (Utilities|Time|ClearTimerbyFunctionName _currentweapon "Primary")))

(event Input|ActionEvents|InputActionSecondary_Fire
  (params (Key :type Key%20Structure))
  (bind _currentweapon (Variables|Default|GetCurrentWeapon))
  (:Pressed
    (Utilities|Time|SetTimerbyFunctionName _currentweapon "Secondary" 0.01 true))
  (:Released
    (Utilities|Time|ClearTimerbyFunctionName _currentweapon "Secondary")))

(event Input|KeyboardEvents|H
  (params (Key :type Key%20Structure))
  (:Released
    (Default|UpgradeWeapon (Variables|Default|GetCurrentWeapon))))

(fn ConstructionScript)

(fn InitWeapon
  (params (Parent :type Scene%20Component%20Object%20Reference) (SocketName :type Name))
  (bind _returnvalue (Game|SpawnActorfromClass "/Game/Blueprints/Weapon/BP_Weapon.BP_Weapon_C" (Math|Transform|MakeTransform "0, 0, 0") "Undefined" 0 0))
  (bind _output_get (Variables|Default|SetCurrentWeapon _returnvalue))
  (Actor|SetOwner _output_get (Game|GetPlayerCharacter 0))
  (Transformation|AttachComponentToComponent _output_get Parent SocketName "KeepRelative" "KeepRelative" "KeepRelative" true)
  (bind _returnvalue_2 (Game|SpawnActorfromClass "/Game/Blueprints/Weapon/BP_NozzleBlow.BP_NozzleBlow_C" (Math|Transform|MakeTransform "0, 0, 0") "Undefined" 0 0))
  (Default|InitNozzle (Variables|Default|GetCurrentWeapon) _returnvalue_2)
  (Transformation|AttachComponentToComponent _returnvalue_2 (Variables|/Game/Blueprints/Weapon/BP_Weapon.BP_Weapon_C|GetWeaponMesh _output_get) "" "KeepRelative" "KeepRelative" "KeepRelative" true))

(fn KilledEnemy
  (params (Matter :type Float%20%28single-precision%29))
  (bind _matterout (Default|ProcessMatter (Variables|Default|GetCurrentWeapon) Matter))
  (Default|ChangeMatterValueby (Variables|Default|GetCurrentVacuumBag) _matterout))

(fn InitVacuumBag
  (params (Parent :type Scene%20Component%20Object%20Reference) (SocketName :type Name))
  (bind _returnvalue (Game|SpawnActorfromClass "/Game/Blueprints/Weapon/BP_VacuumBag.BP_VacuumBag_C" (Math|Transform|MakeTransform "0, 0, 0" "0, 0, 0" "5.000000,5.000000,5.000000") "Undefined" 0 0))
  (bind _output_get (Variables|Default|SetCurrentVacuumBag _returnvalue))
  (Actor|SetOwner _output_get (Game|GetPlayerCharacter 0)))

(fn PushedBack
  (params (Direction :type Vector))
  (Class|CharacterBase|AddImpulsetoCharacterinDirectionwithMagnitude Direction 1e+03)
  (Development|PrintString "Kena pushed"))