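; Player character Blueprint for Babooshka, a swimming grandma with a vacuum weapon in a wave-defense game.
; BeginPlay spawns the weapon and starting nozzle; nozzles can be cycled and leveled, and looping timers drive both fire modes.
; Tick traces from the camera to aim weapon colliders and flag enemies in range.
; It also routes shop and pause input and handles jam, slow and pushback effects; HUD and bag setup calls are disconnected here.
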(event Custom|OnBoostActivated_Event_0
  (params (Charater :type Character%20Base%20Object%20Reference))
  ;[1 1 1] Boost Particle Effect
  (Effects|SpawnEmitterAttached (Variables|Default|GetBoosterParticleSystem) (Variables|/Game/Blueprints/Weapon/BP_VacuumBag.BP_VacuumBag_C|GetVacuumBag (Variables|Default|GetBag_0)) (Variables|Default|GetBoosterEndSocketName) "0, 0, 0" "0, 0, 0" (Variables|Default|GetBoosterParticleScale) "KeepRelativeOffset" true "AutoRelease")
  (Default|PlayBoostSound (Variables|Default|GetBag_0))
  (Variables|Default|SetBoostTimeLeft (Variables|Default|GetBoost_Cooldown)))

(event Custom|SlowedDown
  (params (TempSpeed :type Float%20%28single-precision%29) (Delay :type Float%20%28single-precision%29))
  (bind _mesh (Variables|Character|GetMesh))
  (bind _charactermovement (Variables|Character|GetCharacterMovement))
  ;[1 1 1] Slowing Grandma
  (if (Variables|Default|GetIsSlowed)
    (if (> (Variables|/Script/Engine.CharacterMovementComponent|GetMaxSwimSpeed _charactermovement) TempSpeed)
      (Variables|/Script/Engine.CharacterMovementComponent|SetMaxSwimSpeed _charactermovement TempSpeed :!label _label)
      (bind _returnvalue (Effects|SpawnEmitterAttached "/Game/ParticleEffects/PES_SludgeBubbleSlowing.PES_SludgeBubbleSlowing" _mesh "LeftLegSocket" "0, 0, 0" "0, 0, 0" "0.400000,0.400000,0.400000" "KeepRelativeOffset" true "AutoRelease"))
      (bind _returnvalue_2 (Effects|SpawnEmitterAttached "/Game/ParticleEffects/PES_SludgeBubbleSlowing.PES_SludgeBubbleSlowing" _mesh "RightLegSocket" "0, 0, 0" "0, 0, 0" "0.400000,0.400000,0.400000" "KeepRelativeOffset" true "AutoRelease")))
    (else
      (goto _label)))
  (Utilities|FlowControl|RetriggerableDelay Delay)
  (Variables|/Script/Engine.CharacterMovementComponent|SetMaxSwimSpeed (Variables|Character|GetCharacterMovement) (Variables|Default|GetSwimSpeed))
  (Components|Activation|Deactivate _returnvalue_2)
  (Components|Activation|Deactivate _returnvalue))

(event Custom|JamWeapon
  (params (Duration :type Float%20%28single-precision%29))
  ;[1 1 1] Jam Weapon
  (Variables|Default|SetIsWeaponJammed true)
  (Variables|Default|SetbUseControllerRotationYaw false)
  ;;[1 1 1] Stop Shooting
  (Utilities|Time|ClearTimerbyFunctionName (Variables|Default|GetWeapon) "Primary")
  (Components|Activation|Deactivate (Variables|Default|GetPES_BubbleSucking))
  (Variables|Default|SetIsFiring false)
  (Animation|StopAnimMontage "/Game/Meshes/Characters/Babooshka_Resized/AMontage_Sucking_Babooshka.AMontage_Sucking_Babooshka")
  (Audio|Components|Audio|Stop (Variables|Default|GetWeaponAudio))
  (Utilities|FlowControl|Delay Duration)
  (Variables|Default|SetIsWeaponJammed false))

(event EventBeginPlay
  (CallFunction|InitWeapon))

(event EventPrimaryFireStart
  (bind _weapon (Variables|Default|GetWeapon))
  (Variables|Default|SetbUseControllerRotationYaw true)
  ;[1 1 1] Shoot
  (bind _rateoffire (Default|GetRateOfFire (Variables|/Game/Blueprints/Weapon/BP_Weapon.BP_Weapon_C|GetCurrentNozzle _weapon)))
  (Utilities|Time|SetTimerbyFunctionName _weapon "Primary" _rateoffire true)
  (Components|Activation|Activate (Variables|Default|GetPES_BubbleSucking) false)
  (Variables|Default|SetIsFiring true)
  (Animation|PlayAnimMontage "/Game/Meshes/Characters/Babooshka_Resized/AMontage_Sucking_Babooshka.AMontage_Sucking_Babooshka" 1.0 "Windup")
  (Default|PlayPrimarySound (Variables|Default|GetWeapon)))

(event EventTick
  (params (DeltaSeconds :type Float%20%28single-precision%29))
  (bind _maincamera (Variables|Default|GetMainCamera))
  (bind _returnvalue (Transformation|GetWorldLocation _maincamera))
  (Variables|Default|SetBoostTimeLeft (- (Variables|Default|GetBoostTimeLeft) DeltaSeconds))
  (Variables|Default|SetSecondaryTimeLeft (- (Variables|Default|GetSecondaryTimeLeft) DeltaSeconds))
  ;[1 1 1] Linetrace for Crosshair Enemy Detection
  (bind _outhit (Collision|LineTraceForObjects _returnvalue (+ _returnvalue (* (Math|Vector|GetForwardVector _maincamera) 10000)) (Variables|Default|GetEnemyType) false 0 "None"))
  ;[1 1 1] Set Colliders' Pitch
  (Transformation|SetWorldRotation (Variables|Default|GetWeaponColliders) (Math|Rotator|FindLookatRotation (Transformation|GetWorldLocation (Variables|Character|GetMesh)) (.TraceEnd (|GetActorAndTraceEnd _outhit))) false false)
  (bind _asenemy_base (Utilities|Casting|CastToEnemyBase (.HitActor (|GetActorAndTraceEnd _outhit)))
    (:then
      (bind _result (Default|CheckWithinRange (Variables|Default|GetNozzle) _asenemy_base))
      (Variables|Default|SetIsAnyEnemyInRange _result))
    (:CastFailed
      (Variables|Default|SetIsAnyEnemyInRange false))))

(event EventPrimaryFireEnd
  (Variables|Default|SetbUseControllerRotationYaw false)
  ;[1 1 1] Stop Shooting
  (Utilities|Time|ClearTimerbyFunctionName (Variables|Default|GetWeapon) "Primary")
  (Components|Activation|Deactivate (Variables|Default|GetPES_BubbleSucking))
  (Variables|Default|SetIsFiring false)
  (Animation|StopAnimMontage "/Game/Meshes/Characters/Babooshka_Resized/AMontage_Sucking_Babooshka.AMontage_Sucking_Babooshka")
  (Default|StopPrimarySound (Variables|Default|GetWeapon)))

(event EventSecondaryFireStart
  (if (not (Variables|Default|GetIsFiring))
    (Variables|Default|SetbUseControllerRotationYaw true)
    (Utilities|Time|SetTimerbyFunctionName (Variables|Default|GetWeapon) "Secondary" 0.01 true)))

(event EventSecondaryFireEnd
  (if (Variables|Default|GetIsFiring)
    _
    (else
      (Variables|Default|SetbUseControllerRotationYaw false)))
  (Utilities|Time|ClearTimerbyFunctionName (Variables|Default|GetWeapon) "Secondary"))

(event EventNextEquipment
  (if (Variables|Default|GetIsInUI)
    (bind _shopinventorywidget (Variables|Default|GetShopInventoryWidget)
      (:then
        (Default|NextItemPressed _shopinventorywidget))
      (:else))
    (else
      (CallFunction|GotoNozzleIndex (+ (Variables|Default|GetCurrentNozzleIndex) 1)))))

(event EventPreviousEquipment
  (if (Variables|Default|GetIsInUI)
    (bind _shopinventorywidget (Variables|Default|GetShopInventoryWidget)
      (:then
        (Default|PreviousItemPressed _shopinventorywidget))
      (:else))
    (else
      (CallFunction|GotoNozzleIndex (- (Variables|Default|GetCurrentNozzleIndex) 1)))))

(event EventContextual
  (Utilities|FlowControl|Sequence
    (:then_0
      (bind _asudsgame_mode_base (Utilities|Casting|CastToUDSGameModeBase (Game|GetGameMode)))
      (bind _currentstate (Variables|/Script/UDSTS.UDSGameModeBase|GetCurrentState _asudsgame_mode_base)
        (:then
          (bind _assetup_game_mode_state (Utilities|Casting|CastToSetupGameModeState _currentstate))
          (Variables|/Script/UDSTS.SetupGameModeState|SetfastFoward _assetup_game_mode_state true))
        (:else)))
    (:then_1
      (if (Game|IsGamePaused)
        (bind _aswave_defense_game_state_base (Utilities|Casting|CastToWaveDefenseGameStateBase (Game|GetGameState)))
        (bind _aswidget_pause (Utilities|Casting|CastToWidget_Pause (Variables|/Game/GameModes/WaveDefense/WaveDefenseGameStateBase.WaveDefenseGameStateBase_C|GetPauseWidget _aswave_defense_game_state_base)))
        (Default|OnShareClicked _aswidget_pause)))))

(event Input|ActionEvents|InputActionInteract
  (params (Key :type Key%20Structure))
  (:Pressed
    (if (Variables|Default|GetIsInUI)
      (bind _shopinventorywidget (Variables|Default|GetShopInventoryWidget)
        (:then
          (Default|RepairBasePressed _shopinventorywidget))
        (:else)))))

(event Input|ActionEvents|InputActionConfirm
  (params (Key :type Key%20Structure))
  (:Pressed
    (bind _shopinventorywidget (Variables|Default|GetShopInventoryWidget)
      (:then
        (Default|BuyButtonPressed _shopinventorywidget))
      (:else))))

(event Input|ActionEvents|InputActionExit
  (params (Key :type Key%20Structure))
  (:Pressed
    (Utilities|FlowControl|Sequence
      (:then_0
        (bind _shopinventorywidget (Variables|Default|GetShopInventoryWidget)
          (:then
            (Default|ExitWindowPressed _shopinventorywidget))
          (:else)))
      (:then_1
        (if (Game|IsGamePaused)
          (bind _aswave_defense_game_state_base (Utilities|Casting|CastToWaveDefenseGameStateBase (Game|GetGameState)))
          (bind _aswidget_pause (Utilities|Casting|CastToWidget_Pause (Variables|/Game/GameModes/WaveDefense/WaveDefenseGameStateBase.WaveDefenseGameStateBase_C|GetPauseWidget _aswave_defense_game_state_base)))
          (Default|OnStartClicked _aswidget_pause))))))

(event Input|ActionEvents|InputActionPause
  (params (Key :type Key%20Structure))
  (:Pressed
    (bind _aswave_defense_game_state_base (Utilities|Casting|CastToWaveDefenseGameStateBase (Game|GetGameState)))
    (Default|TogglePause _aswave_defense_game_state_base (not (Game|IsGamePaused)))))

(fn ConstructionScript)

(fn InitWeapon
  (bind _startingnozzle (Variables|Default|GetStartingNozzle))
  (bind _returnvalue (Game|SpawnActorfromClass "/Game/Blueprints/Weapon/BP_Weapon.BP_Weapon_C" (Math|Transform|MakeTransform "0, 0, 0" "0, 0, 0" "0.300000,0.300000,0.300000") "AlwaysSpawn" self 0))
  (bind _output_get (Variables|Default|SetWeapon _returnvalue))
  (Actor|SetOwner _returnvalue 0)
  (Variables|/Game/Blueprints/Weapon/BP_Weapon.BP_Weapon_C|SetCharacter _returnvalue 0)
  (Transformation|AttachComponentToComponent _returnvalue (Variables|Character|GetMesh) (Utilities|Name|MakeLiteralName "weapon_r") "KeepRelative" "KeepRelative" "KeepRelative" true)
  (bind _returnvalue_2 (Game|SpawnActorfromClass (Variables|/Game/Blueprints/Weapon/PDA_Nozzle.PDA_Nozzle_C|GetNozzleClass _startingnozzle) (Math|Transform|MakeTransform "0, 0, 0") "AlwaysSpawn" _returnvalue 0))
  (Default|InitNozzle _output_get _returnvalue_2 _startingnozzle)
  (Utilities|Array|AddUnique (Variables|Default|GetNozzleList) _startingnozzle)
  (Utilities|Map|Add (Variables|Default|GetNozzleToLevelList) _startingnozzle 0)
  (Default|SetNozzleProperties _returnvalue _startingnozzle)
  (Variables|/Game/Blueprints/Weapon/BP_NozzleBase.BP_NozzleBase_C|SetCharacter _returnvalue_2 self)
  (Variables|Default|SetNozzle _returnvalue_2)
  (Transformation|AttachComponentToComponent _returnvalue_2 (Variables|/Game/Blueprints/Weapon/BP_Weapon.BP_Weapon_C|GetWeaponMesh _returnvalue) "nozzle" "KeepRelative" "KeepRelative" "KeepRelative" true))

(fn InitVacuumBag
  (bind _returnvalue (Game|SpawnActorfromClass "/Game/Blueprints/Weapon/BP_VacuumBag.BP_VacuumBag_C" (Math|Transform|MakeTransform "0, 0, 0" "0, 0, 0" "0.400000,0.400000,0.400000") "AlwaysSpawn" self 0))
  (bind _output_get (Variables|Default|SetBag_0 _returnvalue))
  (Actor|SetOwner _output_get self)
  (Transformation|AttachComponentToComponent _output_get (Variables|Character|GetMesh) "Back" "KeepRelative" "KeepRelative" "KeepRelative" true))

(fn KilledEnemy
  (bind _matterout (Default|ProcessMatter (Variables|Default|GetWeapon) 0.0))
  (Default|ChangeMatterValueby (Variables|Default|GetBag_0) _matterout))

(fn TransferNozzle
  (params (IncomingNozzle :type PDA%20Nozzle%20Object%20Reference))
  (bind _nozzletolevellist (Variables|Default|GetNozzleToLevelList))
  (bind _nozzlelist (Variables|Default|GetNozzleList))
  (bind _nozzlelist_2 (Variables|Default|GetNozzleList))
  (bind _returnvalue (Utilities|Array|FindItem _nozzlelist_2 IncomingNozzle))
  (bind _value (Utilities|Map|Find _nozzletolevellist IncomingNozzle))
  (if (Utilities|Array|ContainsItem _nozzlelist IncomingNozzle)
    ;[1 1 1] Adds 1 level to Nozzle
    (if (Utilities|Map|Contains _nozzletolevellist IncomingNozzle)
      (Utilities|Map|Add _nozzletolevellist IncomingNozzle (+ _value 1))
      (CallFunction|GotoNozzleIndex _returnvalue)
      (Default|SetNozzleProperties (Variables|Default|GetWeapon) IncomingNozzle _value)
      (else
        ;[1 1 1] Insert Nozzle
        (Utilities|Map|Add _nozzletolevellist IncomingNozzle 0 :!label _label)
        (CallFunction|GotoNozzleIndex _returnvalue)
        (Default|SetNozzleProperties (Variables|Default|GetWeapon) IncomingNozzle)))
    (else
      (Utilities|Array|AddUnique _nozzlelist IncomingNozzle)
      (goto _label))))

(fn SwitchNozzle
  (params (NewNozzle :type PDA%20Nozzle%20Object%20Reference))
  (bind _nozzletolevellist (Variables|Default|GetNozzleToLevelList))
  (bind (_value _returnvalue) (Utilities|Map|Find _nozzletolevellist NewNozzle))
  (if _returnvalue
    (Default|SetNozzleProperties (Variables|Default|GetWeapon) NewNozzle _value)))

(fn SetupSwitchNozzleWidget
  (bind _asplayer_controller (Utilities|Casting|CastToPlayerController (Pawn|GetController self)))
  (bind _returnvalue (UserInterface|CreateWidget "/Game/Widget/SplitScreen/WBP_NozzleSwitch_Player1.WBP_NozzleSwitch_Player1_C" _asplayer_controller))
  (bind _output_get (Variables|Default|SetNozzleSwitchWidget _returnvalue))
  (Variables|/Game/Widget/SplitScreen/WBP_NozzleSwitch_Player1.WBP_NozzleSwitch_Player1_C|SetPlayer _output_get 0)
  (UserInterface|Viewport|AddtoPlayerScreen _returnvalue 200))

(fn GotoNozzleIndex
  (params (ToIndex :type Integer))
  (bind _nozzlelist (Variables|Default|GetNozzleList))
  (bind _returnvalue (Utilities|Array|Length _nozzlelist))
  (bind _output_get (LocalVariables|SetOldIndex (Variables|Default|GetCurrentNozzleIndex)))
  (if (>= ToIndex _returnvalue)
    (LocalVariables|SetNewIndex 0)
    (elif (< ToIndex 0)
      (LocalVariables|SetNewIndex (- _returnvalue 1))
      (else
        (bind _output_get_2 (LocalVariables|SetNewIndex ToIndex)))))
  (CallFunction|SwitchNozzle (Utilities|Array|Get(acopy) _nozzlelist (LocalVariables|GetNewIndex)))
  (Variables|Default|SetCurrentNozzleIndex _output_get_2)
  (Default|CallOnNozzleIndexChange _output_get))

(fn PushedBack
  (params (Direction :type Vector) (Intensity :type Float%20%28single-precision%29))
  (bind _returnvalue (* Direction Intensity))
  (Physics|AddImpulse (Variables|Character|GetCharacterMovement) _returnvalue true)
  (Effects|SpawnEmitteratLocation "/Game/ParticleEffects/PES_Pushed.PES_Pushed" (Transformation|GetActorLocation) (Math|Conversions|RotationFromXVector _returnvalue)))

(fn DealingDamage
  (Variables|Default|SetIsDealingDamage true)
  (Utilities|Time|SetTimerbyFunctionName 0 "SetFalseDealingDamage" 0.5))

(fn SetFalseDealingDamage
  (Variables|Default|SetIsDealingDamage false))

(fn ClearWeaponTimers
  (bind _weapon (Variables|Default|GetWeapon))
  (Utilities|Time|ClearTimerbyFunctionName _weapon "Secondary")
  (Utilities|Time|ClearTimerbyFunctionName _weapon "Primary")
  (Components|Activation|Deactivate (Variables|Default|GetPES_BubbleSucking))
  (Variables|Default|SetIsFiring false)
  (Animation|StopAnimMontage "/Game/Meshes/Characters/Babooshka_Resized/AMontage_Sucking_Babooshka.AMontage_Sucking_Babooshka")
  (Default|StopPrimarySound (Variables|Default|GetWeapon))
  (Default|StopShootEvent (Variables|Default|GetCrosshairWidget)))