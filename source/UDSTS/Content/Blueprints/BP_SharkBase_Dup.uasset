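; BP_SharkBase_Dup is a shark base actor that enemies and toxic projectiles can strike, destroyed when its health component reports death.
; Overlaps on its damage trigger collider identify BP_EnemyBase or BP_ToxicProjectile, call ApplyDamage with that actor's Damage value, then destroy it.
; Only the enemy branch sets the base itself as the damaged actor; the projectile branch leaves that target unset.
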(event OnComponentBeginOverlap(DamageTriggerCollider)
  (params (OverlappedComponent :type Primitive%20Component%20Object%20Reference) (OtherActor :type Actor%20Object%20Reference) (OtherComp :type Primitive%20Component%20Object%20Reference) (OtherBodyIndex :type Integer) (bFromSweep :type Boolean) (SweepResult :type Hit%20Result%20Structure%20%28by%20ref%29))
  (bind _asbp_enemy_base (Utilities|Casting|CastToBP_EnemyBase OtherActor)
    (:then
      (Game|Damage|ApplyDamage self (Variables|/Script/UDSTS.EnemyBase|GetDamage _asbp_enemy_base) 0 _asbp_enemy_base "/Script/Engine.DamageType")
      (Actor|DestroyActor _asbp_enemy_base))
    (:CastFailed
      (bind _asbp_toxic_projectile (Utilities|Casting|CastToBP_ToxicProjectile OtherActor))
      (Game|Damage|ApplyDamage 0 (Variables|/Game/Blueprints/Enemies/ToxicBlob/BP_ToxicProjectile.BP_ToxicProjectile_C|GetDamage _asbp_toxic_projectile) 0 _asbp_toxic_projectile "/Script/Engine.DamageType")
      (Actor|DestroyActor _asbp_toxic_projectile))))

(event OnDeathEvent(HealthComponent)
  (params (Victim :type Actor%20Object%20Reference) (Killer :type Actor%20Object%20Reference))
  (Actor|DestroyActor))

(event EventBeginPlay)

(event Collision|EventActorBeginOverlap
  (params (OtherActor :type Actor%20Object%20Reference)))

(event EventTick
  (params (DeltaSeconds :type Float%20%28single-precision%29)))

(fn ConstructionScript)