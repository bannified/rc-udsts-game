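; Test plastic-bottle enemy pawn that runs a behavior tree, spawning a default AI controller if needed.
; Positive damage plays a timeline driving the mesh material's Alpha parameter as a hurt mask, ignoring retriggers until it finishes.
; Tick sets yaw from the floating movement velocity via arctangent plus 180 degrees.
; On death by BP_Babooshka, it adds Matter to the killer's Bag and destroys itself.
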(event OnDeathEvent(HealthComponent)
  (params (Victim :type Actor%20Object%20Reference) (Killer :type Actor%20Object%20Reference))
  (bind _asbp_babooshka (Utilities|Casting|CastToBP_Babooshka Killer))
  (Default|ChangeMatterValueby (Variables|/Game/Blueprints/BP_Babooshka.BP_Babooshka_C|GetBag _asbp_babooshka) (Variables|Default|GetMatter))
  (Actor|DestroyActor))

(event Custom|ApplyHurtMaskEvent
  ;[1 1 1] Hurt Mask Application
  (if (not (Variables|Default|GetIsMaskApplied))
    (Variables|Default|SetIsMaskApplied true)
    (bind _data (Timeline|[0,%201,%200] PlayFromStart)
      (:Update
        (Rendering|Material|SetScalarParameterValueonMaterials (Variables|Default|GetMainMesh) "Alpha" _data))
      (:Finished
        (Variables|Default|SetIsMaskApplied false)))))

(event Custom|OnTakeAnyDamage_Event_1
  (params (DamagedActor :type Actor%20Object%20Reference) (Damage :type Float%20%28single-precision%29) (DamageType :type Damage%20Type%20Object%20Reference) (InstigatedBy :type Controller%20Object%20Reference) (DamageCauser :type Actor%20Object%20Reference))
  ;[1 1 1] Bind HurtEvent
  (if (> Damage 0.0)
    (CallFunction|ApplyHurtMaskEvent)))

(event EventBeginPlay
  (bind _self self)
  (bind _returnvalue (AI|GetAIController _self))
  (Utilities|IsValid _returnvalue
    (:Is%20Valid
      (AI|RunBehaviorTree _returnvalue (Variables|Default|GetUnitBehaviorTreeAsset)))
    (:Is%20Not%20Valid
      (Pawn|SpawnDefaultController)
      (bind _asaicontroller (Utilities|Casting|CastToAIController (Pawn|GetController)))
      (AI|RunBehaviorTree _asaicontroller (Variables|Default|GetUnitBehaviorTreeAsset))))
  ;[1 1 1] Bind HurtEvent
  (EventDispatchers|AssignOnTakeAnyDamage (delegate Custom|OnTakeAnyDamage_Event_1)))

(event Collision|EventActorBeginOverlap
  (params (OtherActor :type Actor%20Object%20Reference)))

(event EventTick
  (params (DeltaSeconds :type Float%20%28single-precision%29))
  (bind _floatingpawnmovement (Variables|Default|GetFloatingPawnMovement))
  (bind _velocity (Variables|/Script/Engine.MovementComponent|GetVelocity _floatingpawnmovement))
  (if (!= (.y _velocity) 0.0)
    (Transformation|SetActorRotation (Math|Vector|RotatorfromAxisandAngle "0, 0,1.000000" (+ (Class|KismetMathLibrary|DegAtan (/ (.y _velocity) (.x _velocity))) 1.8e+02)) true)))

(fn ConstructionScript)