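; Game mode state for the setup phase before a wave, part of a prototype state machine built from spawned actors.
; Init takes a wave layout and its setup time, then the state tick accumulates time until that runs out or X is held to skip.
; It then spawns a BP_GMS_Wave, passes it the layout and tells BP_UDSGameModeBase to switch to it.
; The state destroys itself on exit.
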(event EventBeginPlay)

(event EventTick
  (params (DeltaSeconds :type Float%20%28single-precision%29)))

(event EventOnStateTick
  (params (GameMode :type UDS%20Game%20Mode%20Base%20Object%20Reference) (DeltaTime :type Float%20%28single-precision%29))
  (bind _output_get (Variables|Default|SetRunningTime (+ DeltaTime (Variables|Default|GetRunningTime))))
  (if (or (>= _output_get (Variables|Default|GetSetupTime)) (Game|Player|IsInputKeyDown (Game|GetPlayerController 0) "X"))
    (CallFunction|TransitiontoWave GameMode)))

(event EventOnStateEnter
  (params (GameMode :type UDS%20Game%20Mode%20Base%20Object%20Reference))
  (Development|PrintString (Utilities|String|Append (Utilities|GetObjectName self) " OnStateEnter Called!")))

(event EventOnStateStart
  (params (GameMode :type UDS%20Game%20Mode%20Base%20Object%20Reference))
  (Development|PrintString (Utilities|String|Append (Utilities|GetObjectName self) " OnStateStart Called!")))

(event EventOnStateStop
  (params (GameMode :type UDS%20Game%20Mode%20Base%20Object%20Reference)))

(event EventOnStateExit
  (params (GameMode :type UDS%20Game%20Mode%20Base%20Object%20Reference))
  (Actor|DestroyActor))

(fn ConstructionScript)

(fn Init
  (params (WaveLayout :type Wave%20Layout%20Structure))
  (bind _output_get (Variables|Default|SetUpcomingWave WaveLayout))
  (Variables|Default|SetSetupTime (.setuptime _output_get))
  (Variables|Default|SetRunningTime 0.0))

(fn TransitiontoWave
  (params (GameMode :type UDS%20Game%20Mode%20Base%20Object%20Reference))
  (bind _returnvalue (Game|SpawnActorfromClass "/Game/GameModePrototype/GameModeStatesPrototype/BP_GMS_Wave.BP_GMS_Wave_C" (Math|Transform|MakeTransform "0, 0, 0") "Undefined" 0 0))
  (bind _asbp_udsgame_mode_base (Utilities|Casting|CastToBP_UDSGameModeBase GameMode))
  (Default|Init _returnvalue (Variables|Default|GetUpcomingWave))
  (Default|ChangetoState _asbp_udsgame_mode_base _returnvalue))