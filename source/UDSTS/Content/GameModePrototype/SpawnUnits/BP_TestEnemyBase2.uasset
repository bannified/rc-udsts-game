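; Test enemy unit Blueprint that runs an AI behavior tree and removes itself shortly after spawning.
; On BeginPlay it casts its controller to AIController, runs the assigned behavior tree asset, prints its name, then destroys itself after a fixed delay.
; A failed cast only prints a debug message.
; A disconnected node chain for rotating toward the AI focus actor never runs.
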(event EventBeginPlay
  (bind _asaicontroller (Utilities|Casting|CastToAIController (Pawn|GetController self))
    (:then
      (AI|RunBehaviorTree _asaicontroller (Variables|Default|GetUnitBehaviorTreeAsset))
      (Development|PrintString (Utilities|GetDisplayName self))
      (Utilities|FlowControl|Delay 1e+01)
      (Actor|DestroyActor))
    (:CastFailed
      (Development|PrintString "Aicontroller failed"))))

(event Collision|EventActorBeginOverlap
  (params (OtherActor :type Actor%20Object%20Reference)))

(event EventTick
  (params (DeltaSeconds :type Float%20%28single-precision%29)))

(fn ConstructionScript)